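; BP_Pistol is a pistol customization actor with swappable finish, red dot sight and suppressor, driven by an on-screen menu.
; On BeginPlay it creates WBP_MainUI, binds its change events, switches the view to the first CineCameraActor found and enables the cursor with Game and UI input.
; Index-based handlers swap the body material between black and tan, and set or clear the attachment meshes to show or hide them.
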(event EventBeginPlay
  (bind _returnvalue (Game|GetPlayerController 0))
  (CallFunction|UISetup)
  (bind _outactors (Actor|GetAllActorsOfClass "/Script/CinematicCamera.CineCameraActor"))
  (Game|Player|SetViewTargetwithBlend (Game|GetPlayerController 0) (Utilities|Array|Get(acopy) _outactors) 0.0 "VTBlend_Linear" 0.0 false)
  (Variables|/Script/Engine.PlayerController|SetbShowMouseCursor _returnvalue true)
  (Input|SetInputModeGameandUI _returnvalue 0 "DoNotLock" true))

(event EventTick
  (params (DeltaSeconds :type Float%20%28single-precision%29)))

(fn ConstructionScript)

(fn UISetup
  (bind _returnvalue (UserInterface|CreateWidget "/Game/Pistol/UI/Widgets/WBP_MainUI.WBP_MainUI_C" (Game|GetPlayerController 0)))
  (UserInterface|Viewport|AddtoViewport _returnvalue 0)
  (EventDispatchers|BindEventtoTextureChanged _returnvalue (EventDispatchers|CreateEvent :!event TextureChanged))
  (EventDispatchers|BindEventtoScopeChanged _returnvalue (EventDispatchers|CreateEvent :!event ScopeChanged))
  (EventDispatchers|BindEventtoSupressorChanged _returnvalue (EventDispatchers|CreateEvent :!event SuppressorChanged)))

(fn ScopeChanged
  (params (Idx :type Integer))
  (bind _reddot (Variables|Default|GetReddot))
  (switch int Idx
    (:0
      (Components|StaticMesh|SetStaticMesh _reddot "/Game/Pistol/Meshes/SM_Reddot.SM_Reddot"))
    (:1
      (Components|StaticMesh|SetStaticMesh _reddot 0))))

(fn TextureChanged
  (params (Idx :type Integer))
  (bind _baseweapon (Variables|Default|GetBaseWeapon))
  (switch int Idx
    (:0
      (Rendering|Material|SetMaterial _baseweapon 0 "/Game/Pistol/Materials/MI_Pistol_Black.MI_Pistol_Black"))
    (:1
      (Rendering|Material|SetMaterial _baseweapon 0 "/Game/Pistol/Materials/MI_Pistol_Tan.MI_Pistol_Tan"))))

(fn SuppressorChanged
  (params (Idx :type Integer))
  (bind _supressor (Variables|Default|GetSupressor))
  (switch int Idx
    (:0
      (Components|StaticMesh|SetStaticMesh _supressor "/Game/Pistol/Meshes/SM_Supressor.SM_Supressor"))
    (:1
      (Components|StaticMesh|SetStaticMesh _supressor 0))))