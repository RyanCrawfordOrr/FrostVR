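; Drivable multiplayer VR vehicle with driver, shotgun, rear shotgun and turret seats.
; Seat buttons seat or stand characters on the server, which multicasts input binding and updates ownership for the driver.
; VR drivers use lever throttle with auto-brake and curved wheel steering, while non-VR drivers use input axes.
; Exits project onto navmesh and trace to the floor, and leaving the seated head threshold fades the camera.
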(event OnWasUsed(ThrottleLever)
  (Development|PrintString "Hello"))

(event OnButtonStateChanged(ShotgunEnterButton)
  (params (ButtonState :type Boolean) (InteractingActor :type Actor%20Object%20Reference) (InteractingComponent :type Primitive%20Component%20Object%20Reference))
  ;[1 1 1] Handle Shotgun
  (CallFunction|HandleExitButton ButtonState (Variables|Default|GetShotgunAttachment) (Variables|Default|GetShotGunExitLocation) (Variables|Passengers|GetShotgun) (Variables|Default|GetShotgunEnterButton)))

(event OnButtonStateChanged(TurretEnterButton)
  (params (ButtonState :type Boolean) (InteractingActor :type Actor%20Object%20Reference) (InteractingComponent :type Primitive%20Component%20Object%20Reference))
  ;[1 1 1] Handle Turret
  (CallFunction|HandleExitButton ButtonState (Variables|Default|GetTurretAttachment) (Variables|Default|GetTurretExitLocation) (Variables|Passengers|GetGunner) (Variables|Default|GetTurretEnterButton)))

(event OnButtonStateChanged(ShotgunRearEnterButton)
  (params (ButtonState :type Boolean) (InteractingActor :type Actor%20Object%20Reference) (InteractingComponent :type Primitive%20Component%20Object%20Reference))
  ;[1 1 1] Handle Rear Shotgun
  (CallFunction|HandleExitButton ButtonState (Variables|Default|GetShotgunRearAttachment) (Variables|Default|GetShotGunRearExitLocation) (Variables|Passengers|GetShotgunRear) (Variables|Default|GetShotgunRearEnterButton)))

(event OnButtonStateChanged(DriverEnterButton)
  (params (ButtonState :type Boolean) (InteractingActor :type Actor%20Object%20Reference) (InteractingComponent :type Primitive%20Component%20Object%20Reference))
  ;[1 1 1] Handle Driver
  (bind _success (CallFunction|HandleExitButton ButtonState (Variables|Default|GetDriverattachment) (Variables|Default|GetDriverExitLocation) (Variables|Passengers|GetDriver) (Variables|Default|GetDriverEnterButton)))
  (if _success
    (Variables|/Script/VRExpansionPlugin.VRButtonComponent|SetbIsEnabled (Variables|Default|GetStartButton) true)))

(event OnButtonStateChanged(DriverExitButton)
  (params (ButtonState :type Boolean) (InteractingActor :type Actor%20Object%20Reference) (InteractingComponent :type Primitive%20Component%20Object%20Reference))
  ;[1 1 1] Handle Driver
  (bind _success (CallFunction|HandleExitButton (not ButtonState) (Variables|Default|GetDriverattachment) (Variables|Default|GetDriverExitLocation) (Variables|Passengers|GetDriver) (Variables|Default|GetDriverExitButton)))
  (if _success
    (Variables|/Script/VRExpansionPlugin.VRButtonComponent|SetbIsEnabled (Variables|Default|GetStartButton) false)))

(event OnButtonStateChanged(RearShotgunExitButton)
  (params (ButtonState :type Boolean) (InteractingActor :type Actor%20Object%20Reference) (InteractingComponent :type Primitive%20Component%20Object%20Reference))
  ;[1 1 1] Handle Rear Shotgun
  (CallFunction|HandleExitButton (not ButtonState) (Variables|Default|GetShotgunRearAttachment) (Variables|Default|GetShotGunRearExitLocation) (Variables|Passengers|GetShotgunRear) (Variables|Default|GetRearShotgunExitButton)))

(event OnButtonStateChanged(ShotgunExitButton)
  (params (ButtonState :type Boolean) (InteractingActor :type Actor%20Object%20Reference) (InteractingComponent :type Primitive%20Component%20Object%20Reference))
  ;[1 1 1] Handle Shotgun
  (CallFunction|HandleExitButton (not ButtonState) (Variables|Default|GetShotgunAttachment) (Variables|Default|GetShotGunExitLocation) (Variables|Passengers|GetShotgun) (Variables|Default|GetShotgunExitButton)))

(event OnButtonStateChanged(TurretExitButton)
  (params (ButtonState :type Boolean) (InteractingActor :type Actor%20Object%20Reference) (InteractingComponent :type Primitive%20Component%20Object%20Reference))
  ;[1 1 1] Handle Turret
  (CallFunction|HandleExitButton (not ButtonState) (Variables|Default|GetTurretAttachment) (Variables|Default|GetTurretExitLocation) (Variables|Passengers|GetGunner) (Variables|Default|GetTurretExitButton)))

(event Custom|CharacterTakingControl
  (params (Character :type Character%20Object%20Reference) (IsTaking :type Boolean) (Attachment :type Scene%20Component%20Object%20Reference) (RelativeTransformToSeat :type Transform) (InitialCameraTransform :type Transform))
  ;[1 1 1] Server sided setup of seating - also calls multicast to inform everyone that there is a new sitting client
  (CallFunction|NotifyPlayerEnteredVehicle Character IsTaking)
  (bind _asvrbase_character (Utilities|Casting|CastToVRBaseCharacter Character))
  (Class|VRBaseCharacter|ServerSetSeatedMode _asvrbase_character Attachment IsTaking (Class|VRExpansionFunctionLibrary|ToTransformNetQuantize(Transform) RelativeTransformToSeat) (Class|VRExpansionFunctionLibrary|ToTransformNetQuantize(Transform) InitialCameraTransform) 7e+01 2e+01 true "C_MOVE_Walking")
  (if IsTaking
    (if (== Attachment (Variables|Default|GetDriverattachment))
      (bind _astemplate_vr_player_controller (Utilities|Casting|CastToTemplate_VR_Player_Controller (Pawn|GetController _asvrbase_character)))
      (Variables|Default|SetDriverIsInVR (Variables|/Game/VRE/Core/Template_VR_Player_Controller.Template_VR_Player_Controller_C|GetHMDEnabled _astemplate_vr_player_controller)))))

(event Custom|OnSeatedThresholdChanged
  (params (bIsWithinThreshold :type Boolean) (ToThresholdScaler :type Float%20%28single-precision%29))
  (if (Pawn|IsLocallyControlled (Variables|Default|GetLocalChar))
    (if bIsWithinThreshold
      ;[1 1 1] Set up input binding - if only binding to driver we could run this owner only instead of multicast. But this car binds to everyones input
      (if (Variables|Default|GetIsFadingCamera)
        (CameraFades|StopCameraFade (Game|GetPlayerCameraManager 0))
        (Variables|Default|SetIsFadingCamera false))
      (else
        (Class|PlayerCameraManager|SetManualCameraFade :self (Game|GetPlayerCameraManager 0) :InFadeAmount ToThresholdScaler)
        (Variables|Default|SetIsFadingCamera true)))))

(event Custom|NotifyPlayerEnteredVehicle
  (params (Character :type Character%20Object%20Reference) (IsEntering :type Boolean))
  ;[1 1 1] Set up input binding - if only binding to driver we could run this owner only instead of multicast. But this car binds to everyones input
  (if (Pawn|IsLocallyControlled Character)
    (bind _asvrbase_character (Utilities|Casting|CastToVRBaseCharacter Character))
    (Variables|Default|SetLocalChar _asvrbase_character)
    (if IsEntering
      (Class|VRWheeledVehicle|SetBindtoInput (Pawn|GetController _asvrbase_character) true)
      (EventDispatchers|BindEventtoOnSeatThreshholdChangedBind _asvrbase_character (delegate Custom|OnSeatedThresholdChanged))
      (else
        (Class|VRWheeledVehicle|SetBindtoInput (Pawn|GetController _asvrbase_character) false)
        (EventDispatchers|UnbindEventfromOnSeatThreshholdChangedBind _asvrbase_character (delegate Custom|OnSeatedThresholdChanged))
        (if (Variables|Default|GetIsFadingCamera)
          (CameraFades|StopCameraFade (Game|GetPlayerCameraManager 0))
          (Variables|Default|SetIsFadingCamera false))))))

(event Input|EnhancedActionEvents|EnhancedInputActionMoveForward
  (params (ActionValue :type Float%20%28double-precision%29) (ElapsedSeconds :type Float%20%28double-precision%29) (TriggeredSeconds :type Float%20%28double-precision%29) (InputAction :type Input%20Action%20Object%20Reference :default "/Game/VRE/Input/Actions/FPSActions/MoveForward.MoveForward"))
  (bind _vehiclemovementcomponent (Variables|Default|GetVehicleMovementComponent))
  ;[1 1 1] Non VR characters Steering
  (:Triggered
    (if (Math|Boolean|ANDBoolean (not (Variables|Default|GetDriverIsInVR)) (Pawn|IsLocallyControlled (Variables|Default|GetLocalChar)) (Utilities|IsValid (.Character (Utilities|Struct|BreakPassengerInfo (Variables|Passengers|GetDriver))))) :!label _label
      (Class|ChaosVehicleMovementComponent|SetThrottleInput _vehiclemovementcomponent (Math|Float|Absolute(Float) ActionValue))
      (Class|ChaosVehicleMovementComponent|SetTargetGear _vehiclemovementcomponent (Math|Integer|SelectInt -1 1 (< ActionValue 0.0)) true)))
  (:Completed
    (goto _label)))

(event Input|EnhancedActionEvents|EnhancedInputActionMoveRight
  (params (ActionValue :type Float%20%28double-precision%29) (ElapsedSeconds :type Float%20%28double-precision%29) (TriggeredSeconds :type Float%20%28double-precision%29) (InputAction :type Input%20Action%20Object%20Reference :default "/Game/VRE/Input/Actions/FPSActions/MoveRight.MoveRight"))
  ;[1 1 1] Non VR characters Steering
  (:Triggered
    (if (Math|Boolean|ANDBoolean (not (Variables|Default|GetDriverIsInVR)) (Pawn|IsLocallyControlled (Variables|Default|GetLocalChar)) (Utilities|IsValid (.Character (Utilities|Struct|BreakPassengerInfo (Variables|Passengers|GetDriver))))) :!label _label
      (Class|ChaosVehicleMovementComponent|SetSteeringInput (Variables|Default|GetVehicleMovementComponent) ActionValue)))
  (:Completed
    (goto _label)))

(event EventBeginPlay)

(event EventTick
  (params (DeltaSeconds :type Float%20%28single-precision%29))
  (bind _localchar (Variables|Default|GetLocalChar))
  (bind _throttlelever (Variables|Default|GetThrottleLever))
  (bind _vehiclemovementcomponent (Variables|Default|GetVehicleMovementComponent))
  (bind _bisheld (Variables|/Script/VRExpansionPlugin.VRLeverComponent|GetbIsHeld _throttlelever))
  ;[1 1 1] Update
  (Utilities|IsValid _localchar
    (:Is%20Valid
      (Utilities|FlowControl|Sequence
        (:then_0
          (if (Pawn|IsLocallyControlled _localchar)
            (Utilities|IsValid (.Character (Utilities|Struct|BreakPassengerInfo (Variables|Passengers|GetDriver)))
              (:Is%20Valid
                (Utilities|FlowControl|Sequence
                  (:then_0
                    (if (Variables|Default|GetDriverIsInVR)
                      (if _bisheld
                        (CallFunction|AddThrottleInput)
                        (CallFunction|AddSteeringInput)
                        (else
                          (Class|ChaosVehicleMovementComponent|SetThrottleInput _vehiclemovementcomponent 0.0)
                          (Class|ChaosVehicleMovementComponent|SetBrakeInput _vehiclemovementcomponent 1.0)))
                      (Variables|/Script/VRExpansionPlugin.VRButtonComponent|SetbIsEnabled (Variables|Default|GetDriverEnterButton) (not _bisheld))))
                  (:then_2
                    (Rendering|Components|TextRender|SetText (Variables||Display|GetInCarSpeed) (Utilities|Text|ToText(String) (Utilities|String|Append (Utilities|String|ToString(Integer) (CallFunction|GetSpeedinMPH)) " MPH")) :!label _label))))
              (:Is%20Not%20Valid
                (goto _label)))
            (else
              (goto _label))))))))

(event Input|ActionEvents|InputActionAlternateGripLeft
  (params (Key :type Key%20Structure))
  (bind _localchar (Variables|Default|GetLocalChar))
  ;[1 1 1] Re-zero
  (:Pressed
    (Utilities|IsValid _localchar
      (:Is%20Valid
        (Class|VRBaseCharacter|ServerReZeroSeating _localchar (Class|VRExpansionFunctionLibrary|MakeTransformNetQuantize "0, 0, 0" "0, 0, 0" "1,1,1") (Class|VRExpansionFunctionLibrary|ToTransformNetQuantize(Transform) (Transformation|GetRelativeTransform (Variables|/Script/VRExpansionPlugin.VRBaseCharacter|GetVRReplicatedCamera _localchar))) true)))))

(fn ConstructionScript
  (Transformation|AttachComponentToComponent (Variables|Default|GetTurretExitButton) (Variables|Character|GetMesh) "B_Guardian_TurretSocket" "KeepRelative" "KeepRelative" "KeepRelative" false))

(fn UpdateHUDStrings
  (bind _vehiclemovementcomponent (Variables|Default|GetVehicleMovementComponent))
  ;[1 1 1] Setup String for Speed
  (Variables|Display|SetSpeed%20Display%20String (Utilities|String|Append (Utilities|String|ToString(Integer) (Math|Float|Floor (Math|Float|Absolute(Float) (* (Vehicle|GetForwardSpeed _vehiclemovementcomponent) 0.036)))) " km/h"))
  ;[1 1 1] Setup string for Gear
  (LocalVariables|SetCurrentGear (Class|ChaosVehicleMovementComponent|GetCurrentGear _vehiclemovementcomponent))
  (if (Variables|Game|GetInReverseGear) ; If zero display N else display R
    (Variables|Display|SetGear%20Display%20String "R")
    (elif (> (LocalVariables|GetCurrentGear) 0) ; If the gear is above zero use that
      (Variables|Display|SetGear%20Display%20String (Utilities|String|ToString(Integer) (LocalVariables|GetCurrentGear)))
      (else
        (Variables|Display|SetGear%20Display%20String "N")))))

(fn AddThrottleInput
  (bind _vehiclemovementcomponent (Variables|Default|GetVehicleMovementComponent))
  (bind _vehiclemovementcomponent_2 (Variables|Default|GetVehicleMovementComponent))
  (bind _throttlelever (Variables|Default|GetThrottleLever))
  (bind _returnvalue (Vehicle|GetForwardSpeed _vehiclemovementcomponent_2))
  (bind _currentleverangle (Variables|/Script/VRExpansionPlugin.VRLeverComponent|GetCurrentLeverAngle _throttlelever))
  (bind _returnvalue_2 (Math|Float|Absolute(Float) _currentleverangle))
  (if (> _returnvalue_2 (Variables|Default|GetThrottleDeadZone))
    (if (> _currentleverangle 0.0)
      (LocalVariables|SetThrottleInput (/ _currentleverangle (Variables|/Script/VRExpansionPlugin.VRLeverComponent|GetLeverLimitPositive _throttlelever)))
      (else
        (LocalVariables|SetThrottleInput (* (/ (Variables|/Script/VRExpansionPlugin.VRLeverComponent|GetLeverLimitNegative _throttlelever) _returnvalue_2) -1.0))))
    (if (and (> (Math|Float|Absolute(Float) _returnvalue) 1e+01) (!= (Math|Float|Sign(Float) _returnvalue) (Math|Float|Sign(Float) (LocalVariables|GetThrottleInput))))
      ;[1 1 1] Changing direction
      (Class|ChaosVehicleMovementComponent|SetBrakeInput _vehiclemovementcomponent (Math|Float|Absolute(Float) (LocalVariables|GetThrottleInput)))
      (Class|ChaosVehicleMovementComponent|SetThrottleInput _vehiclemovementcomponent 0.0)
      (else
        ;[1 1 1] Actively Throttling
        (Class|ChaosVehicleMovementComponent|SetThrottleInput _vehiclemovementcomponent (Math|Float|Absolute(Float) (LocalVariables|GetThrottleInput)))
        (Class|ChaosVehicleMovementComponent|SetTargetGear _vehiclemovementcomponent (Math|Integer|SelectInt -1 1 (< (LocalVariables|GetThrottleInput) 0.0)) true)
        (Class|ChaosVehicleMovementComponent|SetBrakeInput _vehiclemovementcomponent 0.0)))
    (else
      ;[1 1 1] Inside dead zone
      (Class|ChaosVehicleMovementComponent|SetThrottleInput _vehiclemovementcomponent 0.0)
      (Class|ChaosVehicleMovementComponent|SetBrakeInput _vehiclemovementcomponent 1.0))))

(fn AddSteeringInput
  (bind _steeringwheel (Variables|Default|GetSteeringWheel))
  (bind _currentleverangle (Variables|/Script/VRExpansionPlugin.VRLeverComponent|GetCurrentLeverAngle _steeringwheel))
  (bind _returnvalue (Math|Float|Absolute(Float) _currentleverangle))
  (bind _returnvalue_2 (/ _returnvalue 1.2e+02))
  (Class|ChaosVehicleMovementComponent|SetSteeringInput (Variables|Default|GetVehicleMovementComponent) (* (Math|Float|Clamp(Float) (* _returnvalue_2 (+ _returnvalue_2 0.1))) (Math|Float|Sign(Float) _currentleverangle))))

(fn GetTeleportLocation
  (params (ExitMarker :type Scene%20Component%20Object%20Reference) (Actor :type VR%20Base%20Character%20Object%20Reference))
  (bind _returnvalue (Class|VRBaseCharacter|GetVRLocation Actor))
  (bind _returnvalue_2 (Transformation|GetWorldLocation ExitMarker))
  (bind (_projectedlocation _returnvalue_3) (AI|Navigation|ProjectPointtoNavigation _returnvalue_2 0 0 "400.000000,400.000000,200.000000"))
  (bind _output_get (LocalVariables|SetProjectedLoc _projectedlocation))
  (if (Math|Boolean|ANDBoolean (Math|Vector|NotEqual(Vector) _returnvalue_2 _output_get 0.0001) _returnvalue_3 (Math|Vector|NotEqual(Vector) _projectedlocation "0, 0, 0" 0.0001))
    _
    (else
      (LocalVariables|SetProjectedLoc _returnvalue)))
  (bind _outhit (Collision|LineTraceForObjects (LocalVariables|GetProjectedLoc) (+ (LocalVariables|GetProjectedLoc) "0, 0,-200.000000") (Utilities|Array|MakeArray "ObjectTypeQuery1") false (Utilities|Array|MakeArray Actor) "None")) ; Trace down to find a valid location for player to stand at (original NavMesh location is offset upwards, so we must find the actual floor)
  (return (Math|Vector|SelectVector (.ImpactPoint (Collision|BreakHitResult _outhit)) (- _returnvalue (Math|Vector|MakeVector 0.0 0.0 (Components|Capsule|GetScaledCapsuleHalfHeight (Variables|/Script/Engine.Character|GetCapsuleComponent Actor)))) (.bBlockingHit (Collision|BreakHitResult _outhit)))))

(fn GetSpeedinMPH
  (return (Math|Float|Truncate (Class|ChaosVehicleMovementComponent|GetForwardSpeedMPH (Variables|Default|GetVehicleMovementComponent)))))

(fn SitPlayerDown
  (params (Attachment :type Scene%20Component%20Object%20Reference) (Character :type VR%20Base%20Character%20Object%20Reference) (PassengerInfo :type Passenger%20Info%20Structure%20%28by%20ref%29))
  (bind _vrreplicatedcamera (Variables|/Script/VRExpansionPlugin.VRBaseCharacter|GetVRReplicatedCamera Character))
  (Utilities|IsValid Character
    (:Is%20Valid
      (Utilities|Struct|SetmembersinPassengerInfo PassengerInfo Character (Variables|/Script/Engine.SceneComponent|GetRelativeLocation _vrreplicatedcamera))
      (CallFunction|CharacterTakingControl Character true Attachment (Math|Transform|MakeTransform "0.000000,0.000000,20.000000") (Transformation|GetRelativeTransform _vrreplicatedcamera))
      (Actor|Tick|SetActorTickEnabled true)
      (Math|Integer|IncrementInt (Variables|Passengers|GetPassengerCount)
        (:%20%20
          (if (== Attachment (Variables|Default|GetDriverattachment))
            (Actor|SetOwner Character)
            (Class|VRWheeledVehicle|SetOverrideController (Pawn|GetController Character))))))))

(fn StandPlayerUp
  (params (Attachment :type Scene%20Component%20Object%20Reference) (ExitLocation :type Scene%20Component%20Object%20Reference) (Passenger%20Info :type Passenger%20Info%20Structure%20%28by%20ref%29))
  (bind _character (Utilities|Struct|BreakPassengerInfo Passenger%20Info))
  (Utilities|IsValid _character
    (:Is%20Valid
      (CallFunction|CharacterTakingControl _character false ExitLocation (Math|Transform|MakeTransform (CallFunction|GetTeleportLocation ExitLocation _character) (Transformation|GetWorldRotation ExitLocation)))
      (Math|Integer|DecrementInt (Variables|Passengers|GetPassengerCount)
        (:%20%20
          (Utilities|Struct|SetmembersinPassengerInfo Passenger%20Info))))
    (:Is%20Not%20Valid
      _))
  (if (== Attachment (Variables|Default|GetDriverattachment))
    (Class|ChaosVehicleMovementComponent|SetThrottleInput (Variables|Default|GetVehicleMovementComponent) 0.0)
    (Actor|SetOwner 0)
    (Class|VRWheeledVehicle|SetOverrideController)
    (Variables|Default|SetLocalChar 0)))

(fn HasPassengers
  (return (> (Variables|Passengers|GetPassengerCount) 0)))

(fn OnRepPassengerCount
  (Actor|Tick|SetActorTickEnabled (CallFunction|HasPassengers)))

(fn HandleExitButton
  (params (ButtonState :type Boolean) (Attachment :type Scene%20Component%20Object%20Reference) (ExitLocation :type Scene%20Component%20Object%20Reference) (PassengerInfo :type Passenger%20Info%20Structure%20%28by%20ref%29) (Button :type VR%20Button%20Component%20Object%20Reference))
  (bind _localinteractingcomponent (Variables|/Script/VRExpansionPlugin.VRButtonComponent|GetLocalInteractingComponent Button))
  (Networking|SwitchHasAuthority
    (:Authority
      (if ButtonState
        (Utilities|IsValid (.Character (Utilities|Struct|BreakPassengerInfo PassengerInfo))
          (:Is%20Valid
            _)
          (:Is%20Not%20Valid
            (Utilities|IsValid _localinteractingcomponent
              (:Is%20Valid
                (bind _asvrbase_character (Utilities|Casting|CastToVRBaseCharacter (Components|GetOwner _localinteractingcomponent))
                  (:then
                    (CallFunction|SitPlayerDown Attachment _asvrbase_character PassengerInfo)
                    (return true))
                  (:CastFailed
                    _)))
              (:Is%20Not%20Valid
                _))))
        (else
          (CallFunction|StandPlayerUp Attachment ExitLocation PassengerInfo)
          (Class|VRButtonComponent|SetButtonState Button false true false)
          (return true))))
    (:Remote
      _))
  (return false))