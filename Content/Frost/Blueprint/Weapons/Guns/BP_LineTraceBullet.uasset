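; Simulated bullet for Frost's guns that uses timed line traces instead of a moving projectile to damage VR characters.
; On BeginPlay it precomputes a gravity-curved path up to a maximum flight time, then traces one segment per step interval until something is hit.
; A hit on a living character applies damage, plays a sound for headshots, triggers hit or death handling and gun markers, then destroys the bullet.
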(event EventBeginPlay
  (Variables|Default|SetVelocity (* (Variables|Default|GetBulletSpeed) (Variables|Default|GetForwardVector)))
  (Variables|Default|SetTime 0.0)
  (Utilities|Array|Clear (Variables|Default|GetStartCordinates))
  (Utilities|Array|Clear (Variables|Default|GetEndCordinates))
  (while (<= (Variables|Default|GetTime) (Variables|Default|GetMaxSimulationTime))
    (Variables|Default|SetPreviousLocation (Variables|Default|GetCurrentLocation))
    (bind _output_get (Variables|Default|SetVelocity (Math|Vector|MakeVector (.x (Variables|Default|GetVelocity)) (.y (Variables|Default|GetVelocity)) (- (.z (Variables|Default|GetVelocity)) (* (Variables|Default|GetGravity) (Variables|Default|GetStepInterval))))))
    (Variables|Default|SetCurrentLocation (+ (Variables|Default|GetCurrentLocation) (* _output_get (Variables|Default|GetStepInterval))))
    (Utilities|Array|Add (Variables|Default|GetStartCordinates) (Variables|Default|GetPreviousLocation))
    (Utilities|Array|Add (Variables|Default|GetEndCordinates) (Variables|Default|GetCurrentLocation))
    (Variables|Default|SetTime (+ (Variables|Default|GetTime) (Variables|Default|GetStepInterval))))
  (bind (_array_element _array_index) (Utilities|ForEachLoopwithBreakandDelay (Variables|Default|GetStartCordinates) (Variables|Default|GetStepInterval) :!label _label)
    (:LoopBody
      ;[1 1 1] Update Condition
      (bind (_outhit _returnvalue) (Collision|LineTraceByChannel _array_element (Utilities|Array|Get(acopy) (Variables|Default|GetEndCordinates) _array_index) "TraceTypeQuery1" false (Variables|Default|GetIgnoreActorArray) "ForDuration" true "(R=1.000000,G=0.000000,B=0.000000,A=1.000000)" "(R=0.000000,G=1.000000,B=0.000000,A=1.000000)" 0.1))
      (Variables|Default|SetHitSurface? _returnvalue)
      (Variables|Default|SetHitResult _outhit)
      (if (Variables|Default|GetHitSurface?)
        (goto _label Break)))
    (:Completed
      (Variables|Default|SetHit%20Bone%20Name (.HitBoneName (Collision|BreakHitResult (Variables|Default|GetHitResult))))
      (Variables|Default|SetImpact%20Point (.ImpactPoint (Collision|BreakHitResult (Variables|Default|GetHitResult))))
      (Variables|Default|SetHitmarkerSpawnTransform (Math|Transform|MakeTransform (.ImpactPoint (Collision|BreakHitResult (Variables|Default|GetHitResult)))))
      (bind _asbp_vrcharacter_frost_base (Utilities|Casting|CastToBP_VRCharacter_Frost_Base (.HitActor (Collision|BreakHitResult (Variables|Default|GetHitResult)))))
      (Variables|Default|SetHitPlayerActorRef _asbp_vrcharacter_frost_base)
      (if (> (Variables|/Game/Frost/Blueprint/Character/Core/BP_VRCharacter_Frost_Base.BP_VRCharacter_Frost_Base_C|GetHealth _asbp_vrcharacter_frost_base) 0) ; check if the player is not\nalready daead
        (if (== (Variables|Default|GetHit%20Bone%20Name) (Variables|Default|GetHeadBone)) ; headshot
          (Audio|PlaySoundatLocation (Variables|Default|GetHeadshotSound) (Variables|Default|GetImpact%20Point) "0, 0, 0" 1.0 1.2 0.0 "/Game/VRE/Core/Character/WeaponFireAtten.WeaponFireAtten" 0 0 0))
        (bind _output_get_2 (Variables|/Game/Frost/Blueprint/Character/Core/BP_VRCharacter_Frost_Base.BP_VRCharacter_Frost_Base_C|SetHealth (Variables|Default|GetHitPlayerActorRef) (- (Variables|/Game/Frost/Blueprint/Character/Core/BP_VRCharacter_Frost_Base.BP_VRCharacter_Frost_Base_C|GetHealth (Variables|Default|GetHitPlayerActorRef)) (Variables|Default|GetDamage))))
        (if (<= _output_get_2 0)
          (Default|HandlePlayerDeath (Variables|Default|GetHitPlayerActorRef))
          (Default|SpawnDeathmarkerOwningClient (Variables|Default|GetGunRef) (Variables|Default|GetHitmarkerSpawnTransform))
          (else
            (Default|HandleHitmarkerOwningClient (Variables|Default|GetGunRef) (Variables|Default|GetHitmarkerSpawnTransform))
            (Default|HandlePlayerHit (Variables|Default|GetHitPlayerActorRef))))
        (Actor|DestroyActor)))))

(event Collision|EventActorBeginOverlap
  (params (OtherActor :type Actor%20Object%20Reference)))

(event EventTick
  (params (DeltaSeconds :type Float%20%28single-precision%29)))

(fn ConstructionScript)