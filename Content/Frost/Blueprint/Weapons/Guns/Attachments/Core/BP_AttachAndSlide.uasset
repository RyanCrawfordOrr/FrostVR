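; VR weapon attachment slot that holds a magazine or attachment on a grippable slider and detaches it when slid out.
; Gripping parents the hand mesh to the slider; either slider end hides the mesh and spawns the item, passing remaining ammo to magazines.
; Server, multicast and owning-client events sync visibility, ammo and grips.
; Overlap currently only prints the owner's name for held objects; the attach-and-grab logic is disconnected.
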(event OnComponentBeginOverlap(Magazine_BoxCollision)
  (params (OverlappedComponent :type Primitive%20Component%20Object%20Reference) (OtherActor :type Actor%20Object%20Reference) (OtherComp :type Primitive%20Component%20Object%20Reference) (OtherBodyIndex :type Integer) (bFromSweep :type Boolean) (SweepResult :type Hit%20Result%20Structure%20%28by%20ref%29))
  ;[1 1 1] Handle attaching magazine
  (CallFunction|HandleBeginOverlapforAttachment OtherActor))

(event OnDropped(Attachment_VRSlider)
  (params (GrippingController :type Grip%20Motion%20Controller%20Component%20Object%20Reference) (GripInformation :type BP%20Actor%20Grip%20Information%20Structure%20%28by%20ref%29) (bWasSocketed :type Boolean))
  ;[1 1 1] Handle Attach/Detach Hand at slider
  ;;[1 1 1] On dropped
  (bind _vr_char_base_ref (Class|BPIPlayerInteract|GetPlayerSelfRef(Message) (Components|GetOwner GrippingController)))
  (switch Utilities|FlowControl|Switch|SwitchonEControllerHand (Class|GripMotionControllerComponent|GetHandType GrippingController)
    (:Left
      (CallFunction|RemoveHandandSnapBacktoController (Variables|/Game/Frost/Blueprint/Character/Parent/BP_VRCharacter_Frost_Base.BP_VRCharacter_Frost_Base_C|GetHandRoot-Left _vr_char_base_ref) (Variables|/Game/Frost/Blueprint/Character/Parent/BP_VRCharacter_Frost_Base.BP_VRCharacter_Frost_Base_C|GetHandMesh-Left _vr_char_base_ref)))
    (:Right
      (CallFunction|RemoveHandandSnapBacktoController (Variables|/Game/Frost/Blueprint/Character/Parent/BP_VRCharacter_Frost_Base.BP_VRCharacter_Frost_Base_C|GetHandRoot-Right _vr_char_base_ref) (Variables|/Game/Frost/Blueprint/Character/Parent/BP_VRCharacter_Frost_Base.BP_VRCharacter_Frost_Base_C|GetHandMesh-Right _vr_char_base_ref))))
  (Class|VRSliderComponent|ResetInitialSliderLocation (Variables|Default|GetAttachment_VRSlider)))

(event OnSliderHitPoint(Attachment_VRSlider)
  (params (SliderProgressPoint :type Float%20%28single-precision%29))
  ;[1 1 1] Handle Attach/Detach Hand at slider
  ;;[1 1 1] Slider hit point
  (CallFunction|HitPointServer SliderProgressPoint))

(event OnGripped(Attachment_VRSlider)
  (params (GrippingController :type Grip%20Motion%20Controller%20Component%20Object%20Reference) (GripInformation :type BP%20Actor%20Grip%20Information%20Structure%20%28by%20ref%29))
  (bind _hand (Class|GripMotionControllerComponent|GetHandType GrippingController))
  (bind _attachment_vrslider (Variables|Default|GetAttachment_VRSlider))
  ;[1 1 1] Handle Attach/Detach Hand at slider
  ;;[1 1 1] On Gripped
  (bind _vr_char_base_ref (Class|BPIPlayerInteract|GetPlayerSelfRef(Message) (Components|GetOwner GrippingController)))
  (bind _output_get (Variables|Default|SetSliderGrippingCharacter _vr_char_base_ref))
  (switch Utilities|FlowControl|Switch|SwitchonEControllerHand _hand
    (:Left
      (bind _returnvalue (Transformation|AttachComponentToComponent (Variables|/Game/Frost/Blueprint/Character/Parent/BP_VRCharacter_Frost_Base.BP_VRCharacter_Frost_Base_C|GetHandMesh-Left _output_get) _attachment_vrslider "None" "KeepWorld" "KeepWorld" "KeepWorld" false))
      (if _returnvalue
        (Variables|Default|SetSlider%20-%20Hand%20Mesh-%20Left (Variables|/Game/Frost/Blueprint/Character/Parent/BP_VRCharacter_Frost_Base.BP_VRCharacter_Frost_Base_C|GetHandMesh-Left _output_get))
        (Variables|Default|SetMagSliderHandType _hand :!label _label)))
    (:Right
      (bind _returnvalue_2 (Transformation|AttachComponentToComponent (Variables|/Game/Frost/Blueprint/Character/Parent/BP_VRCharacter_Frost_Base.BP_VRCharacter_Frost_Base_C|GetHandMesh-Right _output_get) _attachment_vrslider "None" "KeepWorld" "KeepWorld" "KeepWorld" false))
      (if _returnvalue_2
        (Variables|Default|SetSlider%20-%20Hand%20Mesh-%20Right (Variables|/Game/Frost/Blueprint/Character/Parent/BP_VRCharacter_Frost_Base.BP_VRCharacter_Frost_Base_C|GetHandMesh-Right _output_get))
        (goto _label)))))

(event Custom|Show%20Mag%20%28and%20hide%20old%20grabbed%20mesh%29%20-%20Server
  (params (Overlapped%20Mag%20Ref :type BP%20Ammo%20Base%20Object%20Reference))
  ;[1 1 1] Handle attaching magazine
  (CallFunction|ShowMag(andHideOldGrabbedMesh)-Mulitcast Overlapped%20Mag%20Ref))

(event Custom|UpdateAmmoValuesMulticast
  (params (AmmoGun :type Integer) (MaxAmmoPerMag :type Integer))
  ;[1 1 1] Handle attaching magazine
  (Variables|Default|SetTempAmmoGun AmmoGun)
  (Variables|Default|SetMaxAmmoPerMag MaxAmmoPerMag))

(event Custom|SpawnStarterMagMulticast
  ;[1 1 1] Handle attaching magazine
  (CallFunction|SpawnStarterMagLocal))

(event Custom|HitPointServer
  (params (Point%20Progress :type Float%20%28double-precision%29))
  (bind _slidergrippingcharacter (Variables|Default|GetSliderGrippingCharacter))
  (bind _slidergrippingcharacter_2 (Variables|Default|GetSliderGrippingCharacter))
  (bind _attachment_vrslider (Variables|Default|GetAttachment_VRSlider))
  (bind _slidergrippingcharacter_3 (Variables|Default|GetSliderGrippingCharacter))
  ;[1 1 1] Handle Attach/Detach Hand at slider
  ;;[1 1 1] Slider hit point
  (if (Math|Float|NearlyEqual(Float) Point%20Progress 1.0 0.15) ; if mag is removed
    (Audio|PlaySoundatLocation (Variables|Default|GetDetach%20Sound) (Transformation|GetWorldLocation (Variables|Default|GetMagazine_BoxCollision)) "0, 0, 0" 0.3 1.0 0.0 "/Game/VRE/Core/Character/VOIPAtten.VOIPAtten" 0 0 0 :!label _label)
    (switch Utilities|FlowControl|Switch|SwitchonEControllerHand (Variables|Default|GetMagSliderHandType)
      (:Left
        (CallFunction|DropGripOwningClient (Variables|/Script/VRExpansionPlugin.VRBaseCharacter|GetLeftMotionController (Variables|Default|GetSliderGrippingCharacter)) _attachment_vrslider)
        (CallFunction|RemoveHandandSnapBackOwningClient (Variables|/Game/Frost/Blueprint/Character/Parent/BP_VRCharacter_Frost_Base.BP_VRCharacter_Frost_Base_C|GetHandRoot-Left _slidergrippingcharacter_2) (Variables|Default|GetSlider%20-%20Hand%20Mesh-%20Left))
        (Class|VRSliderComponent|SetSliderProgress _attachment_vrslider 0.5)
        (Class|VRSliderComponent|ResetInitialSliderLocation _attachment_vrslider)
        (CallFunction|ReplicateVisibilityMulticast)
        (CallFunction|HandleSpawningMagazineLocal (Variables|/Game/Frost/Blueprint/Character/Parent/BP_VRCharacter_Frost_Base.BP_VRCharacter_Frost_Base_C|GetMagSpawnLoc-Left _slidergrippingcharacter_3) _slidergrippingcharacter_3 (Variables|Default|GetMagSliderHandType)))
      (:Right
        (CallFunction|DropGripOwningClient (Variables|/Script/VRExpansionPlugin.VRBaseCharacter|GetRightMotionController (Variables|Default|GetSliderGrippingCharacter)) _attachment_vrslider)
        (CallFunction|RemoveHandandSnapBackOwningClient (Variables|/Game/Frost/Blueprint/Character/Parent/BP_VRCharacter_Frost_Base.BP_VRCharacter_Frost_Base_C|GetHandRoot-Right _slidergrippingcharacter_2) (Variables|Default|GetSlider%20-%20Hand%20Mesh-%20Right))
        (Class|VRSliderComponent|SetSliderProgress _attachment_vrslider 0.5)
        (Class|VRSliderComponent|ResetInitialSliderLocation _attachment_vrslider)
        (CallFunction|ReplicateVisibilityMulticast)
        (CallFunction|HandleSpawningMagazineLocal (Variables|/Game/Frost/Blueprint/Character/Parent/BP_VRCharacter_Frost_Base.BP_VRCharacter_Frost_Base_C|GetMagSpawnLoc-Right _slidergrippingcharacter) _slidergrippingcharacter (Variables|Default|GetMagSliderHandType))))
    (Variables|Default|SetHasAttachedObject false)
    (Default|CallAttachmentWasDetached)
    (elif (Math|Float|NearlyEqual(Float) Point%20Progress 0.0 0.15) ; mag is finished sliding to home position
      (goto _label))))

(event Custom|ReplicateVisibilityServer
  ;[1 1 1] Handle Attach/Detach Hand at slider
  ;;[1 1 1] visibility RPC
  (CallFunction|ReplicateVisibilityMulticast))

(event Custom|RemoveHandAndSnapBack_OwningClient
  (params (Root :type Scene%20Component%20Object%20Reference) (HandMesh :type Scene%20Component%20Object%20Reference))
  ;[1 1 1] Handle Attach/Detach Hand at slider
  ;;[1 1 1] Remove and snap back RPC
  (CallFunction|RemoveHandandSnapBacktoController Root HandMesh))

(event Custom|HandleSpawningMagazineLocal
  (params (MagSpawnLocation :type Scene%20Component%20Object%20Reference) (Owner%20%28Player%20Character%29 :type BP%20VR%20Character%20Frost%20Base%20Object%20Reference) (SliderMagHandType :type EControllerHand%20Enum :default "Left"))
  (bind _maxammopermag (Variables|Default|GetMaxAmmoPerMag))
  ;[1 1 1] Handle Attach/Detach Hand at slider
  ;;[1 1 1] Handle spawning magazine in hand
  (Networking|SwitchHasAuthority
    (:Authority
      (bind _returnvalue (Game|SpawnActorfromClass (Variables|Default|GetAttachmentClass) (Math|Transform|MakeTransform (Transformation|GetWorldLocation MagSpawnLocation) (Transformation|GetWorldRotation MagSpawnLocation)) "AlwaysSpawn" "MultiplyWithRoot" Owner%20%28Player%20Character%29 Owner%20%28Player%20Character%29))
      (if (Utilities|ClassIsChildOf 0 "/Game/Frost/Blueprint/Weapons/Ammo/BP_Ammo_Base.BP_Ammo_Base_C")
        (bind _ammo_ref (Class|BPIWeaponInteract|GetAmmoSelfRef(Message) _returnvalue))
        (Utilities|IsValid _ammo_ref
          (:Is%20Valid
            (Variables|/Game/Frost/Blueprint/Weapons/Ammo/BP_Ammo_Base.BP_Ammo_Base_C|SetCurrentAmmo _ammo_ref (Math|Integer|Clamp(Integer) (- (Variables|Default|GetTempAmmoGun) 1) 0 _maxammopermag))
            (Variables|/Game/Frost/Blueprint/Weapons/Ammo/BP_Ammo_Base.BP_Ammo_Base_C|SetMaxAmmo _ammo_ref _maxammopermag)
            (Variables|/Game/Frost/Blueprint/Weapons/Ammo/BP_Ammo_Base.BP_Ammo_Base_C|SetPelletsPerShell _ammo_ref 20)
            (Default|HandleGripMagOwningClient _ammo_ref MagSpawnLocation SliderMagHandType)
            (if (== (Variables|/Game/Frost/Blueprint/Weapons/Ammo/BP_Ammo_Base.BP_Ammo_Base_C|GetCurrentAmmo _ammo_ref) 0)
              (Default|HideBullets _ammo_ref))))))))

(event Custom|RemoveHandAndSnapBackServer
  (params (Root :type Scene%20Component%20Object%20Reference) (HandMesh :type Scene%20Component%20Object%20Reference))
  ;[1 1 1] Handle Attach/Detach Hand at slider
  ;;[1 1 1] Remove and snap back RPC
  (CallFunction|RemoveHandandSnapBackOwningClient Root HandMesh))

(event Custom|Show%20Mag%20%28and%20hide%20old%20grabbed%20mesh%29%20-%20Mulitcast
  (params (Overlapped%20Ammo%20Base :type BP%20Ammo%20Base%20Object%20Reference))
  (bind _staticmeshcomponent (Variables|/Script/Engine.StaticMeshActor|GetStaticMeshComponent Overlapped%20Ammo%20Base))
  (bind _attachment_mesh (Variables|Default|GetAttachment_Mesh))
  ;[1 1 1] Handle attaching magazine
  (Collision|SetCollisionEnabled (Variables|Default|GetAttachment_VRSlider) "QueryOnly")
  (Rendering|SetVisibility _attachment_mesh true false)
  ;;[1 1 1] Update Slider Mesh
  (bind _returnvalue (Components|StaticMesh|SetStaticMesh _attachment_mesh (Variables|/Script/Engine.StaticMeshComponent|GetStaticMesh _staticmeshcomponent)))
  (if _returnvalue
    (Rendering|SetVisibility _attachment_mesh true false)
    (else
      (Development|PrintString "ERROR: Unable to Set Slider's Mesh" false true "(R=1.000000,G=0.000000,B=0.006960,A=1.000000)")))
  ;;[1 1 1] Hide old Magazine Mesh that was gripped before dropping
  (Rendering|SetVisibility _staticmeshcomponent false true)
  (Physics|SetSimulatePhysics _staticmeshcomponent false)
  (Collision|SetCollisionEnabled _staticmeshcomponent "NoCollision"))

(event Custom|Replicate%20Visibility%20Multicast
  ;[1 1 1] Handle Attach/Detach Hand at slider
  ;;[1 1 1] visibility RPC
  (Rendering|SetVisibility (Variables|Default|GetAttachment_Mesh) false true)
  (Collision|SetCollisionEnabled (Variables|Default|GetAttachment_VRSlider) "NoCollision"))

(event Custom|DropGripOwningClient
  (params (Target%20Controller :type Grip%20Motion%20Controller%20Component%20Object%20Reference) (ObjectToDrop :type Object%20Object%20Reference))
  ;[1 1 1] Handle Attach/Detach Hand at slider
  ;;[1 1 1] Drop grip RPC
  (Class|GripMotionControllerComponent|DropObject Target%20Controller ObjectToDrop 0 false "0, 0, 0" "0, 0, 0"))

(event Custom|HandleBeginOverlapForAttachment
  (params (OtherActor :type Actor%20Object%20Reference))
  ;[1 1 1] Handle attaching magazine
  (bind (_holdingcontrollers _bisheld) (Class|VRGripInterface|IsHeld(Message) OtherActor))
  (if _bisheld
    (Development|PrintString (Utilities|GetDisplayName (Components|GetOwner)) true true "(R=0.022907,G=0.087414,B=1.000000,A=1.000000)" 2e+01)))

(event Custom|SpawnStarterMagLocal
  ;[1 1 1] Handle attaching magazine
  (Variables|Default|SetTempAmmoGun (Variables|Default|GetMaxAmmoPerMag))
  (Variables|Default|SetHasAttachedObject true))

(event Custom|Show%20Attachment%20%28and%20hide%20old%20grabbed%20mesh%29%20-%20Server
  (params (Overlapped%20Attachment%20Actor :type Attachment%20Base%20Object%20Reference))
  ;[1 1 1] Handle attaching magazine
  (CallFunction|ShowAttachment(andHideOldGrabbedMesh) Overlapped%20Attachment%20Actor))

(event Custom|Show%20Attachment%20%28and%20hide%20old%20grabbed%20mesh%29
  (params (Target :type Attachment%20Base%20Object%20Reference))
  (bind _attachment_mesh (Variables|Default|GetAttachment_Mesh))
  ;[1 1 1] Handle attaching magazine
  (Collision|SetCollisionEnabled (Variables|Default|GetAttachment_VRSlider) "QueryOnly")
  ;;[1 1 1] Comment
  (bind _returnvalue (Components|StaticMesh|SetStaticMesh _attachment_mesh (Variables|/Script/Engine.StaticMeshComponent|GetStaticMesh (Variables|/Game/Frost/Blueprint/Weapons/Guns/Attachments/Core/AttachmentBase.AttachmentBase_C|GetGrippableStaticMesh Target))))
  (if _returnvalue
    (Rendering|SetVisibility _attachment_mesh true false)
    (else
      (Development|PrintString "ERROR: Unable to Set Slider's Mesh" false true "(R=1.000000,G=0.000000,B=0.006960,A=1.000000)")))
  ;;[1 1 1] Hide Previously gripped attachment actor's mesh
  (Utilities|IsValid Target
    (:Is%20Valid
      (bind _interp_on_attachment_self_ref (Class|BPIAttachement|AttachandSlideSelfRef(Message) (Variables|/Script/Engine.ChildActorComponent|GetChildActor (Variables|/Game/Frost/Blueprint/Weapons/Guns/Attachments/Core/AttachmentBase.AttachmentBase_C|GetAttachAndSlideActor Target))))
      (Rendering|SetVisibility (Variables|BP_AttachAndSlide_C|GetAttachment_Mesh _interp_on_attachment_self_ref) false true)
      (Physics|SetSimulatePhysics (Variables|BP_AttachAndSlide_C|GetAttachment_Mesh _interp_on_attachment_self_ref) false)
      (Collision|SetCollisionEnabled (Variables|BP_AttachAndSlide_C|GetAttachment_Mesh _interp_on_attachment_self_ref) "NoCollision"))))

(event Custom|UpdateAmmoValuesServer
  (params (AmmoGun :type Integer) (MaxAmmoPerMag :type Integer))
  ;[1 1 1] Handle attaching magazine
  (CallFunction|UpdateAmmoValuesMulticast AmmoGun MaxAmmoPerMag))

(event Custom|SpawnStarterMagServer
  ;[1 1 1] Handle attaching magazine
  (CallFunction|SpawnStarterMagMulticast))

(event Custom|DropMagAndGrabSliderOwningClient
  (params (Overlapped%20Actor :type Actor%20Object%20Reference) (Hand :type EControllerHand%20Enum :default "Left"))
  (bind _attachment_vrslider (Variables|Default|GetAttachment_VRSlider))
  (bind _attachment_vrslider_2 (Variables|Default|GetAttachment_VRSlider))
  (bind _attachingcharacter (Variables|Default|GetAttachingCharacter))
  (bind _attachingcharacter_2 (Variables|Default|GetAttachingCharacter))
  (bind _rightmotioncontroller (Variables|/Script/VRExpansionPlugin.VRBaseCharacter|GetRightMotionController _attachingcharacter))
  (bind _leftmotioncontroller (Variables|/Script/VRExpansionPlugin.VRBaseCharacter|GetLeftMotionController _attachingcharacter_2))
  ;[1 1 1] Handle attaching magazine
  (Utilities|IsValid Overlapped%20Actor
    (:Is%20Valid
      (switch Utilities|FlowControl|Switch|SwitchonEControllerHand Hand
        (:Left
          (Utilities|IsValid _attachingcharacter_2
            (:Is%20Valid
              (Class|GripMotionControllerComponent|DropObject _leftmotioncontroller Overlapped%20Actor 0 false "0, 0, 0" "0, 0, 0")
              (Utilities|FlowControl|DelayUntilNextTick)
              (Class|GripMotionControllerComponent|GripObjectbyInterface _leftmotioncontroller _attachment_vrslider_2 (Transformation|GetWorldTransform _attachment_vrslider_2) false "None" "None" false))))
        (:Right
          (Utilities|IsValid _attachingcharacter_2
            (:Is%20Valid
              (Class|GripMotionControllerComponent|DropObject _rightmotioncontroller Overlapped%20Actor 0 false "0, 0, 0" "0, 0, 0")
              (Utilities|FlowControl|DelayUntilNextTick)
              (Class|GripMotionControllerComponent|GripObjectbyInterface _rightmotioncontroller _attachment_vrslider (Transformation|GetWorldTransform _attachment_vrslider) false "None" "None" false))))))))

(fn ConstructionScript)

(fn RemoveHandandSnapBacktoController
  (params (Root :type Scene%20Component%20Object%20Reference) (HandMesh :type Scene%20Component%20Object%20Reference))
  (Transformation|DetachFromComponent HandMesh "KeepWorld" "KeepWorld" "KeepWorld" true)
  (Transformation|AttachComponentToComponent HandMesh Root "None" "SnapToTarget" "SnapToTarget" "SnapToTarget" true))

(fn HandleSetAmmoValues
  (params (AmmoRef :type BP%20Ammo%20Base%20Object%20Reference))
  (bind _currentammo (Variables|/Game/Frost/Blueprint/Weapons/Ammo/BP_Ammo_Base.BP_Ammo_Base_C|GetCurrentAmmo AmmoRef))
  (if (== (Variables|Default|GetTempAmmoGun) 1) ; If bullet in chamber, make sure to account \nfor it when setting ammo count
    (bind _output_get (Variables|Default|SetTempAmmoGun _currentammo))
    (Math|Integer|IncrementInt _output_get
      (:%20%20
        _))
    (else
      (Variables|Default|SetTempAmmoGun _currentammo)))
  (return (Variables|Default|GetTempAmmoGun) (Variables|/Game/Frost/Blueprint/Weapons/Ammo/BP_Ammo_Base.BP_Ammo_Base_C|GetMaxAmmo AmmoRef)))

(fn AttachandSlideSelfRef
  (return self))

(fn GetAttachmentSelfRef
  (return 0))

(fn GetDataTableRowName
  (return "None"))