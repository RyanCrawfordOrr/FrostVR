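; VR game state that records which team owns each capture point objective.
; On BeginPlay it gathers all CapturePoint_New actors and builds parallel boolean arrays for captured status and Red ownership.
; OnCapture updates both arrays at the objective's index for Red or Blue.
; A per-team tally with debug printing is disconnected and never runs, and IsCaptured returns only default values.
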(event EventBeginPlay
  (bind _outactors (Actor|GetAllActorsOfClass "/Game/Frost/Blueprint/CapturePoint/CapturePoint_New.CapturePoint_New_C"))
  (bind _output_get (Variables|Default|SetCapturePoints _outactors))
  (for _array_element _output_get
    (Utilities|Array|Add (Variables|Default|GetObjectiveStatus) false)
    (Utilities|Array|Add (Variables|Default|GetDoesRedOwnObjective) false)))

(event EventOnCapture
  (params (OwningTeam :type ETeam%20Enum :default "NewEnumerator3") (ObjectiveIndex :type Integer))
  (switch Utilities|FlowControl|Switch|SwitchonETeam OwningTeam
    (:NewEnumerator0
      (Utilities|Array|SetArrayElem (Variables|Default|GetObjectiveStatus) ObjectiveIndex true)
      (Utilities|Array|SetArrayElem (Variables|Default|GetDoesRedOwnObjective) ObjectiveIndex true))
    (:NewEnumerator1
      (Utilities|Array|SetArrayElem (Variables|Default|GetObjectiveStatus) ObjectiveIndex true)
      (Utilities|Array|SetArrayElem (Variables|Default|GetDoesRedOwnObjective) ObjectiveIndex false))))

(event EventTick
  (params (DeltaSeconds :type Float%20%28single-precision%29)))

(fn ConstructionScript)

(fn IsCaptured?
  (return false "NewEnumerator3" "NewEnumerator3" 0))