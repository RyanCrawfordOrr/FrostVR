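; VR player state that assigns each player to the blue or red team when play begins.
; On the server, BeginPlay counts blue and red members across the game state's PlayerArray, then picks the smaller team, or a random one on a tie.
; It stores the result in TeamIndex, sets SelectedTeam and prints the index for debugging.
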(event EventBeginPlay
  ;[1 1 1] Select Team
  ;;[1 1 1] loop through player states on server
  (Networking|SwitchHasAuthority
    (:Authority
      (for _array_element (Variables|/Script/Engine.GameStateBase|GetPlayerArray (Game|GetGameState))
        ;;[1 1 1] Count players on each team
        (bind _asvrplayer_state (Utilities|Casting|CastToVRPlayerState _array_element))
        (if (!= (Variables|VRPlayerState_C|GetTeamIndex _asvrplayer_state) -1)
          (if (== (Variables|VRPlayerState_C|GetTeamIndex _asvrplayer_state) 0)
            (Math|Integer|IncrementInt (Variables|Default|GetBlueTeamTotal))
            (elif (== (Variables|VRPlayerState_C|GetTeamIndex _asvrplayer_state) 1)
              (Math|Integer|IncrementInt (Variables|Default|GetRedTeamTotal))))))
      ;;[1 1 1] Select team based on player counts
      ;;;[1 1 1] if teams are equal
      (if (== (Variables|Default|GetBlueTeamTotal) (Variables|Default|GetRedTeamTotal))
        ;;;[1 1 1] randomly select team
        (if (Math|Random|RandomBool)
          (Variables|Default|SetTeamIndex 0)
          (else
            (Variables|Default|SetTeamIndex 1)))
        (else
          ;;;[1 1 1] choose team with least amount of players
          (if (< (Variables|Default|GetBlueTeamTotal) (Variables|Default|GetRedTeamTotal))
            (Variables|Default|SetTeamIndex 0)
            (else
              (Variables|Default|SetTeamIndex 1)))))
      (Variables|Default|SetSelectedTeam true)
      (Development|PrintString (Utilities|String|ToString(Integer) (Variables|Default|GetTeamIndex))))))

(fn ConstructionScript)