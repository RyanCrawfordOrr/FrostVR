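; VR game mode that registers the game server process with AWS GameLift.
; On BeginPlay it initializes the GameLift server SDK with blank WebSocket and fleet parameters, then reports ProcessReady through a Frost process-parameters object carrying the server port and log path.
; On EndPlay it calls ProcessEnding and quits the server if that succeeds.
; SDK failures are printed as strings; login, new-player and Tick events are empty.
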(event EventHandleStartingNewPlayer
  (params (NewPlayer :type Player%20Controller%20Object%20Reference)))

(event EventBeginPlay
  (bind (_success _errortype _errormessage) (Class|GameLiftServerFunctionLibrary|InitSDK5 (Utilities|Struct|MakeAWSGameLiftServerSDKServerParameters)))
  (if _success
    (bind _returnvalue (Game|ConstructObjectfromClass self "/Game/Frost/Blueprint/Core/Frost_AWS_ProcessParameters.Frost_AWS_ProcessParameters_C" (.port (Class|ServerHelper|ServerIPandPort)) (Utilities|Array|MakeArray (Class|ServerHelper|LogFilePath))))
    (bind (_success_2 _errortype_2 _errormessage_2) (Class|GameLiftServerFunctionLibrary|ProcessReady _returnvalue))
    (if (not _success_2)
      (Development|PrintString (Utilities|String|Append (Utilities|String|EnumtoString _errortype_2) ": " _errormessage_2)))
    (else
      (Development|PrintString _errormessage))))

(event EventEndPlay
  (params (EndPlayReason :type EEndPlayReason%20Enum :default "Destroyed"))
  (bind (_success _errortype _errormessage) (Class|GameLiftServerFunctionLibrary|ProcessEnding))
  (if _success
    (Class|ServerHelper|QuitServer false)
    (else
      (Development|PrintString _errormessage))))

(event EventPostLogin
  (params (NewPlayer :type Player%20Controller%20Object%20Reference)))

(event EventTick
  (params (DeltaSeconds :type Float%20%28single-precision%29)))

(fn ConstructionScript)