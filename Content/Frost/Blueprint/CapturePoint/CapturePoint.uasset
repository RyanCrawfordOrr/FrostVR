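; Team capture point for VR characters, owned by red or blue after the majority team holds its sphere for a set time.
; Overlaps update team counts, then Server-to-Multicast-to-Local events start, pause, resume or restart the capture timer, with equal counts meaning contested.
; Tick polls that timer to complete captures, and the zone mesh material shows team and state.
; Tick also turns the icon widget toward the local camera, scaling it with distance.
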(event OnComponentBeginOverlap(Sphere)
  (params (OverlappedComponent :type Primitive%20Component%20Object%20Reference) (OtherActor :type Actor%20Object%20Reference) (OtherComp :type Primitive%20Component%20Object%20Reference) (OtherBodyIndex :type Integer) (bFromSweep :type Boolean) (SweepResult :type Hit%20Result%20Structure%20%28by%20ref%29))
  (bind _alloverlapplayers (Variables|Default|GetAllOverlapPlayers))
  ;[1 1 1] On overlap event
  (Utilities|IsValid OtherActor
    (:Is%20Valid
      (if (Utilities|ClassIsChildOf (Utilities|GetClass OtherActor) "/Script/VRExpansionPlugin.VRCharacter")
        (if (== (Utilities|Array|FindItem _alloverlapplayers OtherActor) -1)
          (bind _asbp_vrcharacter_frost (Utilities|Casting|CastToBP_VRCharacter_Frost_Base OtherActor))
          (bind (_newparam _selectedteam) (Default|GetTeamIndex _asbp_vrcharacter_frost))
          (if _selectedteam
            (if (!= _newparam 0)
              ;;[1 1 1] may not account for player joining or leaving inside a collision
              (Math|Integer|IncrementInt (Variables|Default|GetRedTeamCount)
                (:%20%20
                  _))
              (else
                (Math|Integer|IncrementInt (Variables|Default|GetBlueTeamCount)
                  (:%20%20
                    _))))
            (Utilities|Array|Add _alloverlapplayers OtherActor)
            (CallFunction|TryStartCaptureServer)))))))

(event OnComponentEndOverlap(Sphere)
  (params (OverlappedComponent :type Primitive%20Component%20Object%20Reference) (OtherActor :type Actor%20Object%20Reference) (OtherComp :type Primitive%20Component%20Object%20Reference) (OtherBodyIndex :type Integer))
  (bind _alloverlapplayers (Variables|Default|GetAllOverlapPlayers))
  ;[1 1 1] On overlap event
  (Utilities|IsValid OtherActor
    (:Is%20Valid
      (if (Utilities|ClassIsChildOf (Utilities|GetClass OtherActor) "/Script/VRExpansionPlugin.VRCharacter")
        (if (!= (Utilities|Array|FindItem _alloverlapplayers OtherActor) -1)
          (bind _asbp_vrcharacter_frost (Utilities|Casting|CastToBP_VRCharacter_Frost_Base OtherActor))
          (bind (_newparam _selectedteam) (Default|GetTeamIndex _asbp_vrcharacter_frost))
          (if _selectedteam
            (if (!= _newparam 0)
              ;;[1 1 1] may not account for player joining or leaving inside a collision
              (Math|Integer|DecrementInt (Variables|Default|GetRedTeamCount)
                (:%20%20
                  _))
              (else
                (Math|Integer|DecrementInt (Variables|Default|GetBlueTeamCount)
                  (:%20%20
                    _))))
            (Utilities|Array|RemoveItem _alloverlapplayers OtherActor)
            (CallFunction|CheckPlayersinRangeServer)))))))

(event Custom|TryStartCaptureServer
  ;[1 1 1] Start Capture
  (CallFunction|TryStartCaptureMulticast))

(event Custom|Check%20Players%20in%20Range%20Local
  (bind _capturetimer (Variables|Default|GetCaptureTimer))
  ;[1 1 1] check players in range
  (if (and (== (Variables|Default|GetBlueTeamCount) 0) (== (Variables|Default|GetRedTeamCount) 0))
    (Variables|Default|SetCapturingTeam "NewEnumerator3")
    (Utilities|Time|ClearandInvalidateTimerbyHandle (Variables|Default|GetCaptureTimer))
    (CallFunction|ChangeCapturePointColor (Variables|Default|GetOwningTeam) (Variables|Default|GetIsCaptured))
    (elif (== (Variables|Default|GetBlueTeamCount) (Variables|Default|GetRedTeamCount))
      (Variables|Default|SetPreviousCapturingTeam (Variables|Default|GetCapturingTeam))
      (CallFunction|ChangeCapturePointColor "NewEnumerator4" false)
      (Utilities|Time|PauseTimerbyHandle (Variables|Default|GetCaptureTimer))
      (elif (Variables|Default|GetIsCaptured)
        (if (> (Variables|Default|GetBlueTeamCount) (Variables|Default|GetRedTeamCount))
          (Variables|Default|SetCapturingTeam "NewEnumerator1")
          (else
            (Variables|Default|SetCapturingTeam "NewEnumerator0")))
        (if (and (Variables|Default|GetCheckForCapture) (Utilities|Enum|NotEqual(Enum) (Variables|Default|GetOwningTeam) (Variables|Default|GetCapturingTeam)))
          (CallFunction|ChangeCapturePointColor (Variables|Default|GetCapturingTeam) false)
          (else
            (CallFunction|ChangeCapturePointColor (Variables|Default|GetCapturingTeam) true)))
        (elif (Utilities|Enum|NotEqual(Enum) (Variables|Default|GetOwningTeam) (Variables|Default|GetCapturingTeam))
          (if (> (Variables|Default|GetBlueTeamCount) (Variables|Default|GetRedTeamCount))
            (Variables|Default|SetCapturingTeam "NewEnumerator1")
            (else
              (Variables|Default|SetCapturingTeam "NewEnumerator0")))
          (CallFunction|ChangeCapturePointColor (Variables|Default|GetCapturingTeam) false)
          (if (Utilities|Enum|Equal(Enum) (Variables|Default|GetPreviousCapturingTeam) (Variables|Default|GetCapturingTeam))
            (Utilities|Time|UnpauseTimerbyHandle _capturetimer)
            (else
              (Utilities|Time|ClearandInvalidateTimerbyHandle _capturetimer)
              (Variables|Default|SetPreviousCapturingTeam (Variables|Default|GetCapturingTeam))
              (CallFunction|StartCaptureTimer)))
          (else
            (Development|PrintString "ERROR: Owning Team != Capturing Team" true true "(R=0.000000,G=0.660000,B=1.000000,A=1.000000)" 9e+01)))))))

(event Custom|EndCaptureLocal
  ;[1 1 1] WHen capture is completed
  (Variables|Default|SetCheckForCapture false)
  (switch Utilities|FlowControl|Switch|SwitchonETeam (Variables|Default|GetCapturingTeam)
    (:NewEnumerator0
      (bind _output_get (Variables|Default|SetIsCaptured true))
      (CallFunction|ChangeCapturePointColor "NewEnumerator0" _output_get)
      (Variables|Default|SetOwningTeam "NewEnumerator0"))
    (:NewEnumerator1
      (bind _output_get_2 (Variables|Default|SetIsCaptured true))
      (CallFunction|ChangeCapturePointColor "NewEnumerator1" _output_get_2)
      (Variables|Default|SetOwningTeam "NewEnumerator1")))
  (CallFunction|CheckPlayersinRangeLocal))

(event Custom|EndCaptureMulticast
  ;[1 1 1] WHen capture is completed
  (CallFunction|EndCaptureLocal))

(event Custom|EndCaptureServer
  ;[1 1 1] WHen capture is completed
  (CallFunction|EndCaptureMulticast))

(event Custom|TryStartCaptureLocal
  ;[1 1 1] Start Capture
  (if (> (Utilities|Time|GetTimerRemainingTimebyHandle (Variables|Default|GetCaptureTimer)) 0.0)
    (CallFunction|CheckPlayersinRangeServer)
    (else
      (if (> (Variables|Default|GetBlueTeamCount) (Variables|Default|GetRedTeamCount))
        (Variables|Default|SetCapturingTeam "NewEnumerator1")
        (else
          (Variables|Default|SetCapturingTeam "NewEnumerator0")))
      (if (Utilities|Enum|NotEqual(Enum) (Variables|Default|GetOwningTeam) (Variables|Default|GetCapturingTeam))
        (CallFunction|ChangeCapturePointColor (Variables|Default|GetCapturingTeam) (Variables|Default|GetIsCaptured)))
      (bind _returnvalue (Utilities|Time|SetTimerbyEvent (delegate Custom|Start%20Capture) (Variables|Default|GetTimeToCapture)))
      (Variables|Default|SetCaptureTimer _returnvalue)
      (CallFunction|StartCapture))))

(event Custom|Start%20Capture
  ;[1 1 1] Start Capture
  (Variables|Default|SetCheckForCapture true))

(event Custom|CheckPlayersInRangeMulitcast
  ;[1 1 1] check players in range
  (CallFunction|CheckPlayersinRangeLocal))

(event Custom|CheckPlayersInRangeServer
  ;[1 1 1] check players in range
  (CallFunction|CheckPlayersinRangeMulitcast))

(event Custom|TryStartCaptureMulticast
  ;[1 1 1] Start Capture
  (CallFunction|TryStartCaptureLocal))

(event Custom|StartCaptureTimer
  ;[1 1 1] Start Capture
  (bind _returnvalue (Utilities|Time|SetTimerbyEvent (delegate Custom|Start%20Capture) (Variables|Default|GetTimeToCapture)))
  (Variables|Default|SetCaptureTimer _returnvalue)
  (CallFunction|StartCapture))

(event EventTick
  (params (DeltaSeconds :type Float%20%28single-precision%29))
  (bind _returnvalue (Game|GetPlayerCameraManager 0))
  (bind _widget (Variables|Default|GetWidget))
  (bind _returnvalue_2 (Camera|GetCameraLocation _returnvalue))
  (bind _returnvalue_3 (Transformation|GetWorldLocation _widget))
  ;[1 1 1] Event tick
  (Utilities|FlowControl|Sequence
    (:then_0
      ;[1 1 1] WHen capture is completed
      (if (and (Variables|Default|GetCheckForCapture) (Utilities|Enum|NotEqual(Enum) (Variables|Default|GetOwningTeam) (Variables|Default|GetCapturingTeam)))
        (if (<= (Utilities|Time|GetTimerRemainingTimebyHandle (Variables|Default|GetCaptureTimer)) 0.0)
          (CallFunction|EndCaptureServer))))
    (:then_1
      ;[1 1 1] Comment
      (Utilities|IsValid _returnvalue
        (:Is%20Valid
          (Transformation|SetWorldTransform _widget (Math|Transform|MakeTransform _returnvalue_3 (Math|Rotator|FindLookatRotation _returnvalue_3 _returnvalue_2) (Math|Conversions|ToVector(Float) (/ (Math|Vector|Distance(Vector) _returnvalue_3 _returnvalue_2) 6e+03))) true false))))))

(event EventBeginPlay
  (bind _ascapture_point_widget_1 (Utilities|Casting|CastToCapturePoint_Widget1 (UserInterface|GetWidget (Variables|Default|GetWidget))))
  (Class|Image|SetBrush (Variables|/Game/Frost/Blueprint/CapturePoint/CapturePoint_Widget1.CapturePoint_Widget1_C|GetImage_0 _ascapture_point_widget_1) (Utilities|Struct|MakeSlateBrush "Image" "NoTile" "NoMirror" "(X=32.000000,Y=32.000000)" "(Left=0.000000,Top=0.000000,Right=0.000000,Bottom=0.000000)" "(SpecifiedColor=(R=1.000000,G=1.000000,B=1.000000,A=1.000000),ColorUseRule=UseColor_Specified)" "(CornerRadii=(X=0.000000,Y=0.000000,Z=0.000000,W=1.000000),Color=(SpecifiedColor=(R=0.000000,G=0.000000,B=0.000000,A=0.000000),ColorUseRule=UseColor_Specified),Width=0.000000,RoundingType=HalfHeightRadius,bUseBrushTransparency=False)" (Variables|Default|GetImage))))

(fn ConstructionScript)

(fn ChangeCapturePointColor
  (params (Team :type ETeam%20Enum :default "NewEnumerator3") (IsCaptured :type Boolean))
  (switch Utilities|FlowControl|Switch|SwitchonETeam Team
    (:NewEnumerator3
      (Rendering|Material|SetMaterial (Variables|Default|GetCaptureZoneMesh) 0 "/Game/Frost/Blueprint/CapturePoint/Material/ZoneMesh/Flashing/TeamColor_Neutral_Transparent.TeamColor_Neutral_Transparent"))
    (:NewEnumerator0
      (if IsCaptured
        (Rendering|Material|SetMaterial (Variables|Default|GetCaptureZoneMesh) 0 "/Game/Frost/Blueprint/CapturePoint/Material/ZoneMesh/TeamColor_Solid_Red.TeamColor_Solid_Red")
        (else
          (Rendering|Material|SetMaterial (Variables|Default|GetCaptureZoneMesh) 0 "/Game/Frost/Blueprint/CapturePoint/Material/ZoneMesh/Flashing/TeamColor_Red_Transparent.TeamColor_Red_Transparent"))))
    (:NewEnumerator1
      (if IsCaptured
        (Rendering|Material|SetMaterial (Variables|Default|GetCaptureZoneMesh) 0 "/Game/Frost/Blueprint/CapturePoint/Material/ZoneMesh/TeamColor_Solid_Blue.TeamColor_Solid_Blue")
        (else
          (Rendering|Material|SetMaterial (Variables|Default|GetCaptureZoneMesh) 0 "/Game/Frost/Blueprint/CapturePoint/Material/ZoneMesh/Flashing/TeamColor_Blue_Transparent.TeamColor_Blue_Transparent"))))
    (:NewEnumerator4
      (Rendering|Material|SetMaterial (Variables|Default|GetCaptureZoneMesh) 0 "/Game/Frost/Blueprint/CapturePoint/Material/ZoneMesh/Flashing/TeamColor_Flashing_Base_Inst.TeamColor_Flashing_Base_Inst")))
  (return))