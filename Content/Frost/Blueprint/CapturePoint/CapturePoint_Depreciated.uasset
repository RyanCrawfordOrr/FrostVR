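; Deprecated team capture point actor for a VR game, where red and blue players standing in its sphere contest and take ownership.
; On authority, overlap events and tick recount players per team and multicast the result, which starts, pauses or restarts a capture timer.
; The timer drives a progress widget that rotates and distance-scales toward the local camera.
; A dynamic material shows team color and flashes during capture or contest.
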(event OnComponentBeginOverlap(OverlapSphere)
  (params (OverlappedComponent :type Primitive%20Component%20Object%20Reference) (OtherActor :type Actor%20Object%20Reference) (OtherComp :type Primitive%20Component%20Object%20Reference) (OtherBodyIndex :type Integer) (bFromSweep :type Boolean) (SweepResult :type Hit%20Result%20Structure%20%28by%20ref%29))
  ;[1 1 1] Overlap Events
  (Networking|SwitchHasAuthority
    (:Authority
      (bind (_blueteamtotal _redteamtotal _alloverlapplayerslist) (CallFunction|CountOverlappingPlayers))
      (if (> (Utilities|Array|Length _alloverlapplayerslist) 0)
        (CallFunction|TryStartCaptureMulticast _blueteamtotal _redteamtotal)))))

(event OnComponentEndOverlap(OverlapSphere)
  (params (OverlappedComponent :type Primitive%20Component%20Object%20Reference) (OtherActor :type Actor%20Object%20Reference) (OtherComp :type Primitive%20Component%20Object%20Reference) (OtherBodyIndex :type Integer))
  ;[1 1 1] Overlap Events
  (Networking|SwitchHasAuthority
    (:Authority
      (bind (_blueteamtotal _redteamtotal _alloverlapplayerslist) (CallFunction|CountOverlappingPlayers))
      (if (> (Utilities|Array|Length _alloverlapplayerslist) 0)
        (CallFunction|CheckPlayersinRangeMulitcast _blueteamtotal _redteamtotal)))))

(event Custom|UpdateProgressBarMulticast
  (params (Progress%20 :type Float%20%28double-precision%29) (Value :type Linear%20Color%20Structure))
  ;[1 1 1] Event Tick
  ;;[1 1 1] Update Progress bar
  (Utilities|IsValid (Variables|Default|GetAs%20Capture%20Point%20Widget)
    (:Is%20Valid
      _)
    (:Is%20Not%20Valid
      (Utilities|FlowControl|DelayUntilNextTick)
      (Utilities|IsValid (Variables|Default|GetAs%20Capture%20Point%20Widget)
        (:Is%20Valid
          _)
        (:Is%20Not%20Valid
          (bind _ascapture_point_widget_1 (Utilities|Casting|CastToCapturePoint_Widget1 (UserInterface|GetWidget (Variables|Default|GetWidget))))
          (Variables|Default|SetAs%20Capture%20Point%20Widget _ascapture_point_widget_1)))))
  (Default|SetPercentandColor (Variables|Default|GetAs%20Capture%20Point%20Widget) Progress%20 Value))

(event Custom|Check%20Players%20in%20Range%20Local
  (params (BlueTeamCount :type Integer) (RedTeamCount :type Integer))
  (bind _capturetimer (Variables|Default|GetCaptureTimer))
  ;[1 1 1] check players in range
  (Variables|Default|SetBlueTeamCount BlueTeamCount)
  (bind _output_get (Variables|Default|SetRedTeamCount RedTeamCount))
  (if (and (== _output_get 0) (== BlueTeamCount 0))
    (Variables|Default|SetCapturingTeam "NewEnumerator3")
    (Utilities|Time|ClearandInvalidateTimerbyHandle (Variables|Default|GetCaptureTimer))
    (CallFunction|ChangeCapturePointColor (Variables|Default|GetOwningTeam) (Variables|Default|GetIsCaptured))
    (Variables|Default|SetCheckForCapture false)
    (switch Utilities|FlowControl|Switch|SwitchonETeam (Variables|Default|GetOwningTeam)
      (:NewEnumerator3
        (CallFunction|UpdateProgressBarMulticast 1.0 (Variables|Default|GetNeutralTeamColor)))
      (:NewEnumerator0
        (CallFunction|UpdateProgressBarMulticast 1.0 (Variables|Default|GetRedTeamColor)))
      (:NewEnumerator1
        (CallFunction|UpdateProgressBarMulticast 1.0 (Variables|Default|GetBlueTeamColor)))
      (:NewEnumerator4
        (CallFunction|UpdateProgressBarMulticast 1.0 (Variables|Default|GetContestedTeamColor))))
    (Variables|Default|SetPercentProgress 1.0)
    (elif (== (Variables|Default|GetBlueTeamCount) (Variables|Default|GetRedTeamCount))
      (Variables|Default|SetPreviousCapturingTeam (Variables|Default|GetCapturingTeam))
      (CallFunction|ChangeCapturePointColor "NewEnumerator4" false)
      (Utilities|Time|PauseTimerbyHandle (Variables|Default|GetCaptureTimer))
      (Variables|Default|SetCapturingTeam "NewEnumerator4")
      (elif (Variables|Default|GetIsCaptured)
        (if (> (Variables|Default|GetBlueTeamCount) (Variables|Default|GetRedTeamCount))
          (Variables|Default|SetCapturingTeam "NewEnumerator1")
          (else
            (Variables|Default|SetCapturingTeam "NewEnumerator0")))
        (if (and (Variables|Default|GetCheckForCapture) (Utilities|Enum|NotEqual(Enum) (Variables|Default|GetOwningTeam) (Variables|Default|GetCapturingTeam)))
          (CallFunction|ChangeCapturePointColor (Variables|Default|GetCapturingTeam) false)
          (else
            (CallFunction|ChangeCapturePointColor (Variables|Default|GetCapturingTeam) true)))
        (elif (Utilities|Enum|NotEqual(Enum) (Variables|Default|GetOwningTeam) (Variables|Default|GetCapturingTeam))
          (if (> (Variables|Default|GetBlueTeamCount) (Variables|Default|GetRedTeamCount))
            (Variables|Default|SetCapturingTeam "NewEnumerator1")
            (else
              (Variables|Default|SetCapturingTeam "NewEnumerator0")))
          (CallFunction|ChangeCapturePointColor (Variables|Default|GetCapturingTeam) false)
          (if (Utilities|Enum|Equal(Enum) (Variables|Default|GetPreviousCapturingTeam) (Variables|Default|GetCapturingTeam))
            (Utilities|Time|UnpauseTimerbyHandle _capturetimer)
            (else
              (Utilities|Time|ClearandInvalidateTimerbyHandle _capturetimer)
              (Variables|Default|SetPreviousCapturingTeam (Variables|Default|GetCapturingTeam))
              (CallFunction|StartCaptureTimer)))
          (else
            (Development|PrintString "ERROR: Owning Team != Capturing Team" true true "(R=0.000000,G=0.660000,B=1.000000,A=1.000000)" 9e+01)))))))

(event Custom|EndCaptureMulticast
  ;[1 1 1] End Capture
  (Variables|Default|SetCheckForCapture false)
  (switch Utilities|FlowControl|Switch|SwitchonETeam (Variables|Default|GetCapturingTeam)
    (:NewEnumerator0
      (bind _output_get (Variables|Default|SetIsCaptured true))
      (CallFunction|ChangeCapturePointColor "NewEnumerator0" _output_get)
      (Variables|Default|SetOwningTeam "NewEnumerator0")
      (bind _output_get_2 (Variables|Default|SetPercentProgress 1.0))
      (CallFunction|UpdateProgressBarMulticast _output_get_2 (Variables|Default|GetRedTeamColor)))
    (:NewEnumerator1
      (bind _output_get_3 (Variables|Default|SetIsCaptured true))
      (CallFunction|ChangeCapturePointColor "NewEnumerator1" _output_get_3)
      (Variables|Default|SetOwningTeam "NewEnumerator1")
      (bind _output_get_4 (Variables|Default|SetPercentProgress 1.0))
      (CallFunction|UpdateProgressBarMulticast _output_get_4 (Variables|Default|GetBlueTeamColor)))))

(event Custom|TryStartCaptureLocal
  (params (BlueTeamCount :type Integer) (RedTeamCount :type Integer))
  ;[1 1 1] Start Capture
  (Variables|Default|SetBlueTeamCount BlueTeamCount)
  (Variables|Default|SetRedTeamCount RedTeamCount)
  (if (> (Utilities|Time|GetTimerRemainingTimebyHandle (Variables|Default|GetCaptureTimer)) 0.0)
    (CallFunction|CheckPlayersinRangeMulitcast (Variables|Default|GetBlueTeamCount) (Variables|Default|GetRedTeamCount))
    (else
      (if (> (Variables|Default|GetBlueTeamCount) (Variables|Default|GetRedTeamCount))
        (Variables|Default|SetCapturingTeam "NewEnumerator1")
        (else
          (Variables|Default|SetCapturingTeam "NewEnumerator0")))
      (if (Utilities|Enum|NotEqual(Enum) (Variables|Default|GetOwningTeam) (Variables|Default|GetCapturingTeam))
        (CallFunction|ChangeCapturePointColor (Variables|Default|GetCapturingTeam) (Variables|Default|GetIsCaptured))
        (bind _returnvalue (Utilities|Time|SetTimerbyEvent (delegate Custom|EndOfCaptureTimer) (Variables|Default|GetTimeToCapture)))
        (Variables|Default|SetCaptureTimer _returnvalue)
        (Variables|Default|SetCheckForCapture true)))))

(event Custom|EndOfCaptureTimer
  ;[1 1 1] Start Capture
  (CallFunction|EndCaptureMulticast)
  (Utilities|FlowControl|DelayUntilNextTick)
  (bind (_blueteamtotal _redteamtotal) (CallFunction|CountOverlappingPlayers))
  (CallFunction|CheckPlayersinRangeMulitcast _blueteamtotal _redteamtotal))

(event Custom|CheckPlayersInRangeMulitcast
  (params (BlueTeamCount :type Integer) (RedTeamCount :type Integer))
  ;[1 1 1] check players in range
  (CallFunction|CheckPlayersinRangeLocal BlueTeamCount RedTeamCount))

(event Custom|TryStartCaptureMulticast
  (params (BlueTeamCount :type Integer) (RedTeamCount :type Integer))
  ;[1 1 1] Start Capture
  (CallFunction|TryStartCaptureLocal BlueTeamCount RedTeamCount))

(event Custom|StartCaptureTimer
  ;[1 1 1] Start Capture
  (bind _returnvalue (Utilities|Time|SetTimerbyEvent (delegate Custom|EndOfCaptureTimer) (Variables|Default|GetTimeToCapture)))
  (Variables|Default|SetCaptureTimer _returnvalue)
  (Variables|Default|SetCheckForCapture true))

(event Custom|StartFlashing
  (bind _dynamicmaterial (Variables|Default|GetDynamicMaterial))
  (bind _newtrack_0 (Timeline|Timeline Play)
    (:Update
      (Rendering|Material|SetScalarParameterValue _dynamicmaterial "FadeAmount" _newtrack_0 :!class /Script/Engine.MaterialInstanceDynamic) ; Handle Flashing
      (if (not (Variables|Default|GetCheckForCapture))
        (if (Variables|Default|GetIsCaptured)
          (Timeline|Timeline Stop)
          (else
            (Rendering|Material|SetScalarParameterValue _dynamicmaterial "FadeAmount" (Variables|Default|GetDefaltOpacity) :!class /Script/Engine.MaterialInstanceDynamic)
            (Timeline|Timeline Stop)))))
    (:Finished
      (Timeline|Timeline PlayFromStart))))

(event EventBeginPlay
  ;[1 1 1] Begin Play
  (Utilities|FlowControl|Sequence
    (:then_1
      (bind _ascapture_point_widget_1 (Utilities|Casting|CastToCapturePoint_Widget1 (UserInterface|GetWidget (Variables|Default|GetWidget))))
      (Class|Image|SetBrush (Variables|/Game/Frost/Blueprint/Widget/CapturePoint/CapturePoint_Widget1.CapturePoint_Widget1_C|GetBackgroundImage _ascapture_point_widget_1) (Utilities|Struct|MakeSlateBrush "Image" "NoTile" "NoMirror" "(X=32.000000,Y=32.000000)" "(Left=0.000000,Top=0.000000,Right=0.000000,Bottom=0.000000)" "(SpecifiedColor=(R=1.000000,G=1.000000,B=1.000000,A=1.000000),ColorUseRule=UseColor_Specified)" "(CornerRadii=(X=0.000000,Y=0.000000,Z=0.000000,W=1.000000),Color=(SpecifiedColor=(R=0.000000,G=0.000000,B=0.000000,A=0.000000),ColorUseRule=UseColor_Specified),Width=0.000000,RoundingType=HalfHeightRadius,bUseBrushTransparency=False)" (Variables|Default|GetDefaultObjectiveImage)))
      (Variables|Default|SetAs%20Capture%20Point%20Widget _ascapture_point_widget_1))))

(event EventTick
  (params (DeltaSeconds :type Float%20%28single-precision%29))
  (bind _returnvalue (Game|GetPlayerCameraManager 0))
  (bind _capturetimer (Variables|Default|GetCaptureTimer))
  (bind _timetocapture (Variables|Default|GetTimeToCapture))
  (bind _widget (Variables|Default|GetWidget))
  (bind _returnvalue_2 (Camera|GetCameraLocation _returnvalue))
  (bind _returnvalue_3 (Utilities|Time|GetTimerRemainingTimebyHandle _capturetimer))
  (bind _returnvalue_4 (Transformation|GetWorldLocation _widget))
  (bind _returnvalue_5 (/ _returnvalue_3 _timetocapture))
  (bind _returnvalue_6 (- 1.0 _returnvalue_5))
  (bind _returnvalue_7 (Math|Float|Clamp(Float) _returnvalue_6))
  ;[1 1 1] Event Tick
  ;;[1 1 1] Event tick
  (Utilities|FlowControl|Sequence
    (:then_0
      ;;[1 1 1] check for capture
      (if (Variables|Default|GetCheckForCapture)
        (Utilities|FlowControl|Sequence
          (:then_0
            ;;[1 1 1] Handles  players that may leave the game while on an objective
            (Networking|SwitchHasAuthority
              (:Authority
                (Utilities|FlowControl|Delay 0.5)
                (bind (_blueteamtotal _redteamtotal) (CallFunction|CountOverlappingPlayers))
                (CallFunction|CheckPlayersinRangeMulitcast _blueteamtotal _redteamtotal))))
          (:then_1
            ;;[1 1 1] Update Progress bar
            (Variables|Default|SetPercentProgress _returnvalue_7)
            (Utilities|IsValid (Variables|Default|GetAs%20Capture%20Point%20Widget)
              (:Is%20Valid
                (switch Utilities|FlowControl|Switch|SwitchonETeam (Variables|Default|GetCapturingTeam)
                  (:NewEnumerator0
                    (CallFunction|UpdateProgressBarMulticast _returnvalue_7 (Variables|Default|GetRedTeamColor)))
                  (:NewEnumerator1
                    (CallFunction|UpdateProgressBarMulticast _returnvalue_7 (Variables|Default|GetBlueTeamColor)))
                  (:NewEnumerator4
                    (CallFunction|UpdateProgressBarMulticast _returnvalue_7 (Variables|Default|GetContestedTeamColor))))))))))
    (:then_1
      (Utilities|FlowControl|Delay 0.05)
      ;;[1 1 1] Update rotation to face local player
      (Utilities|IsValid _returnvalue
        (:Is%20Valid
          (Transformation|SetWorldTransform _widget (Math|Transform|MakeTransform _returnvalue_4 (Math|Rotator|FindLookatRotation _returnvalue_4 _returnvalue_2) (Math|Conversions|ToVector(Float) (/ (Math|Vector|Distance(Vector) _returnvalue_4 _returnvalue_2) 6e+03))) true false))))))

(fn ConstructionScript
  (bind _returnvalue (Rendering|Material|CreateDynamicMaterialInstance (Variables|Default|GetCaptureZoneMesh) 0 "/Game/Frost/Material/DepthFade/DepthFade.DepthFade" "None" :!class /Script/Engine.PrimitiveComponent))
  (bind _output_get (Variables|Default|SetDynamicMaterial _returnvalue))
  (Rendering|Material|SetScalarParameterValue _output_get "FadeDistance" 2e+02 :!class /Script/Engine.MaterialInstanceDynamic)
  (Rendering|Material|SetScalarParameterValue _output_get "FadeAmount" (Variables|Default|GetDefaltOpacity) :!class /Script/Engine.MaterialInstanceDynamic))

(fn ChangeCapturePointColor
  (params (Team :type ETeam%20Enum :default "NewEnumerator3") (IsCaptured :type Boolean))
  (bind _dynamicmaterial (Variables|Default|GetDynamicMaterial))
  (bind _blueteamcolor (Variables|Default|GetBlueTeamColor))
  (bind _redteamcolor (Variables|Default|GetRedTeamColor))
  (bind _dynamicmaterial_2 (Variables|Default|GetDynamicMaterial))
  (switch Utilities|FlowControl|Switch|SwitchonETeam Team
    (:NewEnumerator3
      (Rendering|Material|SetVectorParameterValue (Variables|Default|GetDynamicMaterial) "Color" (Variables|Default|GetNeutralTeamColor) :!class /Script/Engine.MaterialInstanceDynamic))
    (:NewEnumerator0
      (if IsCaptured
        (Rendering|Material|SetVectorParameterValue _dynamicmaterial_2 "Color" _redteamcolor :!class /Script/Engine.MaterialInstanceDynamic)
        (Rendering|Material|SetScalarParameterValue _dynamicmaterial_2 "FadeAmount" (Variables|Default|GetCapturedFadeValue) :!class /Script/Engine.MaterialInstanceDynamic)
        (else
          (CallFunction|StartFlashing)
          (Rendering|Material|SetVectorParameterValue (Variables|Default|GetDynamicMaterial) "Color" _redteamcolor :!class /Script/Engine.MaterialInstanceDynamic))))
    (:NewEnumerator1
      (if IsCaptured
        (Rendering|Material|SetVectorParameterValue _dynamicmaterial "Color" _blueteamcolor :!class /Script/Engine.MaterialInstanceDynamic)
        (Rendering|Material|SetScalarParameterValue _dynamicmaterial "FadeAmount" (Variables|Default|GetCapturedFadeValue) :!class /Script/Engine.MaterialInstanceDynamic)
        (else
          (CallFunction|StartFlashing)
          (Rendering|Material|SetVectorParameterValue (Variables|Default|GetDynamicMaterial) "Color" _blueteamcolor :!class /Script/Engine.MaterialInstanceDynamic))))
    (:NewEnumerator4
      (CallFunction|StartFlashing)
      (Rendering|Material|SetVectorParameterValue (Variables|Default|GetDynamicMaterial) "Color" (Variables|Default|GetContestedTeamColor) :!class /Script/Engine.MaterialInstanceDynamic)))
  (return))

(fn OnRepIsCaptured
  (bind _alloverlapplayerslist (CallFunction|CountOverlappingPlayers))
  (if (> (Utilities|Array|Length _alloverlapplayerslist) 0)
    _))

(fn CountOverlappingPlayers
  (Variables|Default|SetBlueTeamCount 0)
  (Variables|Default|SetRedTeamCount 0)
  (Variables|Default|SetAllOverlapPlayers (Utilities|Array|MakeArray 0))
  (for _array_element (Collision|GetOverlappingActors (Variables|Default|GetOverlapSphere) "/Game/Frost/Blueprint/Character/Parent/BP_VRCharacter_Frost_Base.BP_VRCharacter_Frost_Base_C" :!class /Script/Engine.PrimitiveComponent)
    (bind _asbp_vrcharacter_frost_base (Utilities|Casting|CastToBP_VRCharacter_Frost_Base _array_element))
    (bind (_newparam _selectedteam) (Default|GetTeamIndex _asbp_vrcharacter_frost_base))
    (if _selectedteam
      (if (!= _newparam 0)
        (Math|Integer|IncrementInt (Variables|Default|GetRedTeamCount)
          (:%20%20
            _))
        (else
          (Math|Integer|IncrementInt (Variables|Default|GetBlueTeamCount)
            (:%20%20
              _))))
      (Utilities|Array|Add (Variables|Default|GetAllOverlapPlayers) _array_element)))
  (return (Variables|Default|GetBlueTeamCount) (Variables|Default|GetRedTeamCount) (Variables|Default|GetAllOverlapPlayers)))

(fn ChangeCapturePointColorOld
  (params (Team :type ETeam%20Enum :default "NewEnumerator3") (IsCaptured :type Boolean))
  (switch Utilities|FlowControl|Switch|SwitchonETeam Team
    (:NewEnumerator3
      (Rendering|Material|SetMaterial (Variables|Default|GetCaptureZoneMesh) 0 "/Game/Frost/Blueprint/CapturePoint/Material/ZoneMesh/Flashing/TeamColor_Neutral_Transparent.TeamColor_Neutral_Transparent"))
    (:NewEnumerator0
      (if IsCaptured
        (Rendering|Material|SetMaterial (Variables|Default|GetCaptureZoneMesh) 0 "/Game/Frost/Blueprint/CapturePoint/Material/ZoneMesh/TeamColor_Solid_Red.TeamColor_Solid_Red")
        (else
          (Rendering|Material|SetMaterial (Variables|Default|GetCaptureZoneMesh) 0 "/Game/Frost/Blueprint/CapturePoint/Material/ZoneMesh/Flashing/TeamColor_Red_Transparent.TeamColor_Red_Transparent"))))
    (:NewEnumerator1
      (if IsCaptured
        (Rendering|Material|SetMaterial (Variables|Default|GetCaptureZoneMesh) 0 "/Game/Frost/Blueprint/CapturePoint/Material/ZoneMesh/TeamColor_Solid_Blue.TeamColor_Solid_Blue")
        (else
          (Rendering|Material|SetMaterial (Variables|Default|GetCaptureZoneMesh) 0 "/Game/Frost/Blueprint/CapturePoint/Material/ZoneMesh/Flashing/TeamColor_Blue_Transparent.TeamColor_Blue_Transparent"))))
    (:NewEnumerator4
      (Rendering|Material|SetMaterial (Variables|Default|GetCaptureZoneMesh) 0 "/Game/Frost/Blueprint/CapturePoint/Material/ZoneMesh/Flashing/TeamColor_Flashing_Base_Inst.TeamColor_Flashing_Base_Inst")))
  (return))

(fn OnRepCapturingTeam
  (Development|PrintString (Utilities|String|EnumtoString (Variables|Default|GetCapturingTeam)) true true "(R=0.000000,G=0.660000,B=1.000000,A=1.000000)" 2e+02))