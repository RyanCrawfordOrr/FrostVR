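; Team capture point for a VR multiplayer game, where the team with more players in the zone captures it over time.
; The server counts overlapping players via sphere overlaps and delayed tick rechecks, then sets the capturing team.
; RepNotifies start, pause or clear the capture timer and recolor or flash the zone's dynamic material.
; A multicast updates the progress widget, whose transform each character adjusts on tick.
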(event OnComponentBeginOverlap(OverlapSphere)
  (params (OverlappedComponent :type Primitive%20Component%20Object%20Reference) (OtherActor :type Actor%20Object%20Reference) (OtherComp :type Primitive%20Component%20Object%20Reference) (OtherBodyIndex :type Integer) (bFromSweep :type Boolean) (SweepResult :type Hit%20Result%20Structure%20%28by%20ref%29))
  (bind _overlapsphere (Variables|Default|GetOverlapSphere))
  (bind _overlappingactors (Collision|GetOverlappingActors _overlapsphere "/Game/Frost/Blueprint/Character/Parent/BP_VRCharacter_Frost_Base.BP_VRCharacter_Frost_Base_C" :!class /Script/Engine.PrimitiveComponent))
  ;[1 1 1] Overlap Events
  (Networking|SwitchHasAuthority
    (:Authority
      (if (Math|Boolean|ANDBoolean (not (Utilities|Array|ContainsItem (Variables|Default|GetPlayersOnObjective) OtherActor)) (Utilities|ClassIsChildOf (Utilities|GetClass OtherActor) "/Game/Frost/Blueprint/Character/Parent/BP_VRCharacter_Frost_Base.BP_VRCharacter_Frost_Base_C") (Utilities|Array|ContainsItem _overlappingactors OtherActor))
        (bind (_blueteamtotal _redteamtotal _playersonobjective) (CallFunction|CountOverlappingPlayers _overlappingactors))
        (Variables|Default|SetPlayersOnObjective _playersonobjective)
        (Variables|Default|SetBlueTeamCount _blueteamtotal)
        (Variables|Default|SetRedTeamCount _redteamtotal)
        (bind (_capturingteam _both_team_counts_equal_0_ _team_counts_equal_) (CallFunction|GetCapturingTeam _blueteamtotal _redteamtotal))
        (if (not (Utilities|Enum|Equal(Enum) _capturingteam (Variables|Default|GetCapturingTeam)))
          (if (or (Utilities|Enum|Equal(Enum) (Variables|Default|GetCapturingTeam) "NewEnumerator0") (Utilities|Enum|Equal(Enum) (Variables|Default|GetCapturingTeam) "NewEnumerator1")) ; set previous team only to specific team name, not contested or none
            (Variables|Default|SetPreviousCapturingTeam (Variables|Default|GetCapturingTeam)))
          (Variables|Default|SetCapturingTeam _capturingteam)
          (if (Math|Boolean|ANDBoolean (not (> (Utilities|Time|GetTimerRemainingTimebyHandle (Variables|Default|GetCaptureTimer)) 0.0)) (not (Variables|Default|GetIsCaptured)) (not _both_team_counts_equal_0_) (not _team_counts_equal_))
            (CallFunction|StartCaptureTimer)))))))

(event OnComponentEndOverlap(OverlapSphere)
  (params (OverlappedComponent :type Primitive%20Component%20Object%20Reference) (OtherActor :type Actor%20Object%20Reference) (OtherComp :type Primitive%20Component%20Object%20Reference) (OtherBodyIndex :type Integer))
  (bind _overlapsphere (Variables|Default|GetOverlapSphere))
  (bind _overlappingactors (Collision|GetOverlappingActors _overlapsphere "/Game/Frost/Blueprint/Character/Parent/BP_VRCharacter_Frost_Base.BP_VRCharacter_Frost_Base_C" :!class /Script/Engine.PrimitiveComponent))
  ;[1 1 1] Overlap Events
  (Networking|SwitchHasAuthority
    (:Authority
      (if (and (Utilities|Array|ContainsItem (Variables|Default|GetPlayersOnObjective) OtherActor) (not (Utilities|Array|ContainsItem _overlappingactors OtherActor)))
        (bind (_blueteamtotal _redteamtotal _playersonobjective) (CallFunction|CountOverlappingPlayers _overlappingactors))
        (Variables|Default|SetPlayersOnObjective _playersonobjective)
        (Variables|Default|SetBlueTeamCount _blueteamtotal)
        (Variables|Default|SetRedTeamCount _redteamtotal)
        (bind _capturingteam (CallFunction|GetCapturingTeam _blueteamtotal _redteamtotal))
        (if (not (Utilities|Enum|Equal(Enum) _capturingteam (Variables|Default|GetCapturingTeam)))
          (if (or (Utilities|Enum|Equal(Enum) (Variables|Default|GetCapturingTeam) "NewEnumerator0") (Utilities|Enum|Equal(Enum) (Variables|Default|GetCapturingTeam) "NewEnumerator1")) ; set previous team only to specific team name, not contested or none
            (Variables|Default|SetPreviousCapturingTeam (Variables|Default|GetCapturingTeam)))
          (Variables|Default|SetCapturingTeam _capturingteam))))))

(event Custom|UpdateProgressBarMulticast
  (params (Progress%20 :type Float%20%28double-precision%29) (Value :type Linear%20Color%20Structure))
  ;[1 1 1] Event Tick
  ;;[1 1 1] Update Progress bar
  (Utilities|IsValid (Variables|Default|GetAs%20Capture%20Point%20Widget)
    (:Is%20Valid
      _)
    (:Is%20Not%20Valid
      (Utilities|FlowControl|DelayUntilNextTick)
      (Utilities|IsValid (Variables|Default|GetAs%20Capture%20Point%20Widget)
        (:Is%20Valid
          _)
        (:Is%20Not%20Valid
          (bind _ascapture_point_widget_1 (Utilities|Casting|CastToCapturePoint_Widget1 (UserInterface|GetWidget (Variables|Default|GetWidget))))
          (Variables|Default|SetAs%20Capture%20Point%20Widget _ascapture_point_widget_1)))))
  (Default|SetPercentandColor (Variables|Default|GetAs%20Capture%20Point%20Widget) Progress%20 Value))

(event Custom|StartCaptureTimer
  ;[1 1 1] Capture Point Timer
  (bind _returnvalue (Utilities|Time|SetTimerbyEvent (delegate Custom|CaptureTimerEvent) (Variables|Default|GetTimeToCapture)))
  (Variables|Default|SetCaptureTimer _returnvalue)
  (Variables|Default|SetCheckForCapture true))

(event Custom|EndCaptureMulticast
  ;[1 1 1] End Capture
  (Variables|Default|SetCheckForCapture false)
  (switch Utilities|FlowControl|Switch|SwitchonETeam (Variables|Default|GetCapturingTeam)
    (:NewEnumerator0
      (Variables|Default|SetOwningTeam "NewEnumerator0")
      (bind _output_get (Variables|Default|SetPercentProgress 1.0))
      (CallFunction|UpdateProgressBarMulticast _output_get (Variables|Default|GetRedTeamColor)))
    (:NewEnumerator1
      (Variables|Default|SetOwningTeam "NewEnumerator1")
      (bind _output_get_2 (Variables|Default|SetPercentProgress 1.0))
      (CallFunction|UpdateProgressBarMulticast _output_get_2 (Variables|Default|GetBlueTeamColor))))
  (Utilities|FlowControl|Delay 0.2)
  (Variables|Default|SetIsCaptured true))

(event Custom|CaptureTimerEvent
  ;[1 1 1] Capture Point Timer
  (CallFunction|EndCaptureMulticast))

(event Custom|StartFlashing
  (bind _dynamicmaterial (Variables|Default|GetDynamicMaterial))
  ;[1 1 1] Handle Flashing
  (bind _newtrack_0 (Timeline|Timeline Play)
    (:Update
      (Rendering|Material|SetScalarParameterValue _dynamicmaterial "FadeAmount" _newtrack_0 :!class /Script/Engine.MaterialInstanceDynamic) ; Handle Flashing
      (if (not (Variables|Default|GetCheckForCapture))
        (if (Variables|Default|GetIsCaptured)
          (Timeline|Timeline Stop)
          (else
            (Rendering|Material|SetScalarParameterValue _dynamicmaterial "FadeAmount" (Variables|Default|GetDefaltOpacity) :!class /Script/Engine.MaterialInstanceDynamic)
            (Timeline|Timeline Stop)))))
    (:Finished
      (Timeline|Timeline PlayFromStart))))

(event EventBeginPlay
  ;[1 1 1] Begin Play
  (bind _ascapture_point_widget_1 (Utilities|Casting|CastToCapturePoint_Widget1 (UserInterface|GetWidget (Variables|Default|GetWidget))))
  (Class|Image|SetBrush (Variables|/Game/Frost/Blueprint/Widget/CapturePoint/CapturePoint_Widget1.CapturePoint_Widget1_C|GetBackgroundImage _ascapture_point_widget_1) (Utilities|Struct|MakeSlateBrush "Image" "NoTile" "NoMirror" "(X=32.000000,Y=32.000000)" "(Left=0.000000,Top=0.000000,Right=0.000000,Bottom=0.000000)" "(SpecifiedColor=(R=1.000000,G=1.000000,B=1.000000,A=1.000000),ColorUseRule=UseColor_Specified)" "(CornerRadii=(X=0.000000,Y=0.000000,Z=0.000000,W=1.000000),Color=(SpecifiedColor=(R=0.000000,G=0.000000,B=0.000000,A=0.000000),ColorUseRule=UseColor_Specified),Width=0.000000,RoundingType=HalfHeightRadius,bUseBrushTransparency=False)" (Variables|Default|GetDefaultObjectiveImage)))
  (Variables|Default|SetAs%20Capture%20Point%20Widget _ascapture_point_widget_1))

(event EventTick
  (params (DeltaSeconds :type Float%20%28single-precision%29))
  (bind _capturetimer (Variables|Default|GetCaptureTimer))
  (bind _timetocapture (Variables|Default|GetTimeToCapture))
  (bind _returnvalue (Utilities|Time|GetTimerRemainingTimebyHandle _capturetimer))
  (bind _returnvalue_2 (/ _returnvalue _timetocapture))
  (bind _returnvalue_3 (- 1.0 _returnvalue_2))
  (bind _returnvalue_4 (Math|Float|Clamp(Float) _returnvalue_3))
  ;[1 1 1] Event Tick
  ;;[1 1 1] Event tick
  (Utilities|FlowControl|Sequence
    (:then_0
      ;;[1 1 1] check for capture
      (if (Variables|Default|GetCheckForCapture)
        (Utilities|FlowControl|Sequence
          (:then_0
            ;;[1 1 1] Handles  players that may leave the game while on an objective
            (Networking|SwitchHasAuthority
              (:Authority
                (Utilities|FlowControl|Delay 0.5)
                (bind (_blueteamtotal _redteamtotal _playersonobjective) (CallFunction|CountOverlappingPlayers (Collision|GetOverlappingActors (Variables|Default|GetOverlapSphere) "/Game/Frost/Blueprint/Character/Parent/BP_VRCharacter_Frost_Base.BP_VRCharacter_Frost_Base_C" :!class /Script/Engine.PrimitiveComponent)))
                (Variables|Default|SetPlayersOnObjective _playersonobjective)
                (Variables|Default|SetBlueTeamCount _blueteamtotal)
                (Variables|Default|SetRedTeamCount _redteamtotal)
                (bind _capturingteam (CallFunction|GetCapturingTeam _blueteamtotal _redteamtotal))
                (if (not (Utilities|Enum|Equal(Enum) _capturingteam (Variables|Default|GetCapturingTeam)))
                  (if (or (Utilities|Enum|Equal(Enum) (Variables|Default|GetCapturingTeam) "NewEnumerator0") (Utilities|Enum|Equal(Enum) (Variables|Default|GetCapturingTeam) "NewEnumerator1")) ; set previous team only to specific team name, not contested or none
                    (Variables|Default|SetPreviousCapturingTeam (Variables|Default|GetCapturingTeam)))
                  (Variables|Default|SetCapturingTeam _capturingteam)))))
          (:then_1
            ;;[1 1 1] Update Progress bar
            (Networking|SwitchHasAuthority
              (:Authority
                (Variables|Default|SetPercentProgress _returnvalue_4)
                (Utilities|IsValid (Variables|Default|GetAs%20Capture%20Point%20Widget)
                  (:Is%20Valid
                    (switch Utilities|FlowControl|Switch|SwitchonETeam (Variables|Default|GetCapturingTeam)
                      (:NewEnumerator0
                        (CallFunction|UpdateProgressBarMulticast _returnvalue_4 (Variables|Default|GetRedTeamColor)))
                      (:NewEnumerator1
                        (CallFunction|UpdateProgressBarMulticast _returnvalue_4 (Variables|Default|GetBlueTeamColor)))
                      (:NewEnumerator4
                        (CallFunction|UpdateProgressBarMulticast _returnvalue_4 (Variables|Default|GetContestedTeamColor))))))))))))
    (:then_2
      ;;[1 1 1] Update rotation to face local player
      (bind _outactors (Actor|GetAllActorsOfClass "/Game/Frost/Blueprint/Character/Parent/BP_VRCharacter_Frost_Base.BP_VRCharacter_Frost_Base_C"))
      (for _array_element _outactors
        (Default|SetLocalTransformOfUI _array_element (Variables|Default|GetWidget) (.Z (Math|Vector|BreakVector (Transformation|GetWorldLocation (Variables|Default|GetOverlapSphere)))) DeltaSeconds)))))

(fn ConstructionScript
  (bind _returnvalue (Rendering|Material|CreateDynamicMaterialInstance (Variables|Default|GetCaptureZoneMesh) 0 "/Game/Frost/Material/DepthFade/DepthFade.DepthFade" "None" :!class /Script/Engine.PrimitiveComponent))
  (bind _output_get (Variables|Default|SetDynamicMaterial _returnvalue))
  (Rendering|Material|SetScalarParameterValue _output_get "FadeDistance" 2e+02 :!class /Script/Engine.MaterialInstanceDynamic)
  (Rendering|Material|SetScalarParameterValue _output_get "FadeAmount" (Variables|Default|GetDefaltOpacity) :!class /Script/Engine.MaterialInstanceDynamic)
  (bind _ascapture_point_widget_1 (Utilities|Casting|CastToCapturePoint_Widget1 (UserInterface|GetWidget (Variables|Default|GetWidget))))
  (Class|Image|SetBrush (Variables|/Game/Frost/Blueprint/Widget/CapturePoint/CapturePoint_Widget1.CapturePoint_Widget1_C|GetBackgroundImage _ascapture_point_widget_1) (Utilities|Struct|MakeSlateBrush "Image" "NoTile" "NoMirror" "(X=32.000000,Y=32.000000)" "(Left=0.000000,Top=0.000000,Right=0.000000,Bottom=0.000000)" "(SpecifiedColor=(R=1.000000,G=1.000000,B=1.000000,A=1.000000),ColorUseRule=UseColor_Specified)" "(CornerRadii=(X=0.000000,Y=0.000000,Z=0.000000,W=1.000000),Color=(SpecifiedColor=(R=0.000000,G=0.000000,B=0.000000,A=0.000000),ColorUseRule=UseColor_Specified),Width=0.000000,RoundingType=HalfHeightRadius,bUseBrushTransparency=False)" (Variables|Default|GetDefaultObjectiveImage)))
  (Variables|Default|SetAs%20Capture%20Point%20Widget _ascapture_point_widget_1))

(fn ChangeCapturePointColor
  (params (Team :type ETeam%20Enum :default "NewEnumerator3") (IsCaptured :type Boolean))
  (bind _dynamicmaterial (Variables|Default|GetDynamicMaterial))
  (bind _blueteamcolor (Variables|Default|GetBlueTeamColor))
  (bind _redteamcolor (Variables|Default|GetRedTeamColor))
  (bind _dynamicmaterial_2 (Variables|Default|GetDynamicMaterial))
  (switch Utilities|FlowControl|Switch|SwitchonETeam Team
    (:NewEnumerator3
      (Rendering|Material|SetVectorParameterValue (Variables|Default|GetDynamicMaterial) "Color" (Variables|Default|GetNeutralTeamColor) :!class /Script/Engine.MaterialInstanceDynamic))
    (:NewEnumerator0
      (if IsCaptured
        (Rendering|Material|SetVectorParameterValue _dynamicmaterial_2 "Color" _redteamcolor :!class /Script/Engine.MaterialInstanceDynamic)
        (Rendering|Material|SetScalarParameterValue _dynamicmaterial_2 "FadeAmount" (Variables|Default|GetCapturedFadeValue) :!class /Script/Engine.MaterialInstanceDynamic)
        (else
          (CallFunction|StartFlashing)
          (Rendering|Material|SetVectorParameterValue (Variables|Default|GetDynamicMaterial) "Color" _redteamcolor :!class /Script/Engine.MaterialInstanceDynamic))))
    (:NewEnumerator1
      (if IsCaptured
        (Rendering|Material|SetVectorParameterValue _dynamicmaterial "Color" _blueteamcolor :!class /Script/Engine.MaterialInstanceDynamic)
        (Rendering|Material|SetScalarParameterValue _dynamicmaterial "FadeAmount" (Variables|Default|GetCapturedFadeValue) :!class /Script/Engine.MaterialInstanceDynamic)
        (else
          (CallFunction|StartFlashing)
          (Rendering|Material|SetVectorParameterValue (Variables|Default|GetDynamicMaterial) "Color" _blueteamcolor :!class /Script/Engine.MaterialInstanceDynamic))))
    (:NewEnumerator4
      (CallFunction|StartFlashing)
      (Rendering|Material|SetVectorParameterValue (Variables|Default|GetDynamicMaterial) "Color" (Variables|Default|GetContestedTeamColor) :!class /Script/Engine.MaterialInstanceDynamic)))
  (return))

(fn OnRepIsCaptured
  (bind _owningteam (Variables|Default|GetOwningTeam))
  (CallFunction|ChangeCapturePointColor _owningteam (Variables|Default|GetIsCaptured))
  (switch Utilities|FlowControl|Switch|SwitchonETeam _owningteam
    (:NewEnumerator0
      (CallFunction|UpdateProgressBarMulticast 1.0 (Variables|Default|GetRedTeamColor)))
    (:NewEnumerator1
      (CallFunction|UpdateProgressBarMulticast 1.0 (Variables|Default|GetBlueTeamColor))))
  (Variables|Default|SetPercentProgress 1.0))

(fn CountOverlappingPlayers
  (params (OverlapArray :type Array%20of%20Actor%20Object%20References))
  (Utilities|Array|Clear (Variables|Default|GetPlayersOnObjective))
  (LocalVariables|SetLocalRedTeamCount 0)
  (LocalVariables|SetLocalBlueTeamCount 0)
  (for _array_element OverlapArray
    (bind _asbp_vrcharacter_frost_base (Utilities|Casting|CastToBP_VRCharacter_Frost_Base _array_element))
    (bind (_newparam _selectedteam) (Default|GetTeamIndex _asbp_vrcharacter_frost_base))
    (if _selectedteam
      (if (!= _newparam 0)
        (Math|Integer|IncrementInt (LocalVariables|GetLocalRedTeamCount)
          (:%20%20
            _))
        (else
          (Math|Integer|IncrementInt (LocalVariables|GetLocalBlueTeamCount)
            (:%20%20
              _))))
      (Utilities|Array|Add (LocalVariables|GetLocalPlayersOnObjective) _array_element)))
  (return (LocalVariables|GetLocalRedTeamCount) (LocalVariables|GetLocalBlueTeamCount) (LocalVariables|GetLocalPlayersOnObjective)))

(fn ChangeCapturePointColorOld
  (params (Team :type ETeam%20Enum :default "NewEnumerator3") (IsCaptured :type Boolean))
  (switch Utilities|FlowControl|Switch|SwitchonETeam Team
    (:NewEnumerator3
      (Rendering|Material|SetMaterial (Variables|Default|GetCaptureZoneMesh) 0 "/Game/Frost/Blueprint/CapturePoint/Material/ZoneMesh/Flashing/TeamColor_Neutral_Transparent.TeamColor_Neutral_Transparent"))
    (:NewEnumerator0
      (if IsCaptured
        (Rendering|Material|SetMaterial (Variables|Default|GetCaptureZoneMesh) 0 "/Game/Frost/Blueprint/CapturePoint/Material/ZoneMesh/TeamColor_Solid_Red.TeamColor_Solid_Red")
        (else
          (Rendering|Material|SetMaterial (Variables|Default|GetCaptureZoneMesh) 0 "/Game/Frost/Blueprint/CapturePoint/Material/ZoneMesh/Flashing/TeamColor_Red_Transparent.TeamColor_Red_Transparent"))))
    (:NewEnumerator1
      (if IsCaptured
        (Rendering|Material|SetMaterial (Variables|Default|GetCaptureZoneMesh) 0 "/Game/Frost/Blueprint/CapturePoint/Material/ZoneMesh/TeamColor_Solid_Blue.TeamColor_Solid_Blue")
        (else
          (Rendering|Material|SetMaterial (Variables|Default|GetCaptureZoneMesh) 0 "/Game/Frost/Blueprint/CapturePoint/Material/ZoneMesh/Flashing/TeamColor_Blue_Transparent.TeamColor_Blue_Transparent"))))
    (:NewEnumerator4
      (Rendering|Material|SetMaterial (Variables|Default|GetCaptureZoneMesh) 0 "/Game/Frost/Blueprint/CapturePoint/Material/ZoneMesh/Flashing/TeamColor_Flashing_Base_Inst.TeamColor_Flashing_Base_Inst")))
  (return))

(fn GetCapturingTeam
  (params (BlueTeamCount :type Integer) (RedTeamCount :type Integer))
  (LocalVariables|SetLocalBlueTeamCount BlueTeamCount)
  (LocalVariables|SetLocalRedTeamCount RedTeamCount)
  (if (and (== (LocalVariables|GetLocalBlueTeamCount) 0) (== (LocalVariables|GetLocalRedTeamCount) 0))
    (LocalVariables|SetLocalCapturingTeam "NewEnumerator3")
    (elif (== (LocalVariables|GetLocalBlueTeamCount) (LocalVariables|GetLocalRedTeamCount))
      (LocalVariables|SetLocalCapturingTeam "NewEnumerator4")
      (elif (Variables|Default|GetIsCaptured)
        (if (> (LocalVariables|GetLocalBlueTeamCount) (LocalVariables|GetLocalRedTeamCount))
          (LocalVariables|SetLocalCapturingTeam "NewEnumerator1")
          (else
            (LocalVariables|SetLocalCapturingTeam "NewEnumerator0")))
        (elif (> (LocalVariables|GetLocalBlueTeamCount) (LocalVariables|GetLocalRedTeamCount))
          (LocalVariables|SetLocalCapturingTeam "NewEnumerator1")
          (else
            (LocalVariables|SetLocalCapturingTeam "NewEnumerator0"))))))
  (return (LocalVariables|GetLocalCapturingTeam) (and (== (LocalVariables|GetLocalBlueTeamCount) 0) (== (LocalVariables|GetLocalRedTeamCount) 0)) (== (LocalVariables|GetLocalBlueTeamCount) (LocalVariables|GetLocalRedTeamCount))))

(fn OnRepCapturingTeam
  (bind _capturetimer (Variables|Default|GetCaptureTimer))
  (CallFunction|ChangeCapturePointColor (Variables|Default|GetCapturingTeam) (Variables|Default|GetIsCaptured))
  (switch Utilities|FlowControl|Switch|SwitchonETeam (Variables|Default|GetCapturingTeam) ; Handle Timer
    (:NewEnumerator3
      (if (not (Variables|Default|GetIsCaptured))
        (Utilities|Time|ClearandInvalidateTimerbyHandle (Variables|Default|GetCaptureTimer))))
    (:NewEnumerator0
      (if (Utilities|Enum|NotEqual(Enum) (Variables|Default|GetPreviousCapturingTeam) (Variables|Default|GetCapturingTeam)) :!label _label
        (Utilities|Time|ClearandInvalidateTimerbyHandle (Variables|Default|GetCaptureTimer))
        (CallFunction|StartCaptureTimer)
        (else
          (Utilities|Time|UnpauseTimerbyHandle _capturetimer))))
    (:NewEnumerator1
      (goto _label))
    (:NewEnumerator4
      (Utilities|Time|PauseTimerbyHandle _capturetimer))))