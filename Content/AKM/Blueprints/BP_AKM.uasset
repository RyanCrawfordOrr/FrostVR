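; BP_AKM is an AKM rifle customization actor that lets the player swap magazine, scope, handguard and stock through a UI.
; On BeginPlay it creates WBP_MainUI, binds its change events, views through the first CineCamera and enables the mouse cursor.
; Each handler maps the selected index to a skeletal mesh on its component, with empty options clearing the part.
; The scope choice also adds or removes the rail mount.
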(event EventBeginPlay
  (bind _returnvalue (Game|GetPlayerController 0))
  (CallFunction|UISetup)
  (bind _outactors (Actor|GetAllActorsOfClass "/Script/CinematicCamera.CineCameraActor"))
  (Game|Player|SetViewTargetwithBlend (Game|GetPlayerController 0) (Utilities|Array|Get(acopy) _outactors) 0.0 "VTBlend_Linear" 0.0 false)
  (Variables|/Script/Engine.PlayerController|SetbShowMouseCursor _returnvalue true)
  (Input|SetInputModeGameandUI _returnvalue 0 "DoNotLock" true false))

(fn ConstructionScript)

(fn UISetup
  (bind _returnvalue (UserInterface|CreateWidget "/Game/AKM/UI/Widgets/WBP_MainUI.WBP_MainUI_C" (Game|GetPlayerController 0)))
  (UserInterface|Viewport|AddtoViewport _returnvalue 0)
  (EventDispatchers|BindEventtoMagChanged _returnvalue (EventDispatchers|CreateEvent :!event MagChanged))
  (EventDispatchers|BindEventtoScopeChanged _returnvalue (EventDispatchers|CreateEvent :!event ScopeChanged))
  (EventDispatchers|BindEventtoHandguardChanged _returnvalue (EventDispatchers|CreateEvent :!event HandguardChanged))
  (EventDispatchers|BindEventtoStockChanged _returnvalue (EventDispatchers|CreateEvent :!event StockChanged)))

(fn ScopeChanged
  (params (Idx :type Integer))
  (bind _scope (Variables|Default|GetScope))
  (bind _railmount (Variables|Default|GetRailMount))
  (switch int Idx
    (:0
      (Components|SkinnedMesh|SetSkinnedAssetandUpdate _scope "/Game/AKM/Meshes/Parts/SK_ACOG_Scope.SK_ACOG_Scope" true)
      (Components|SkinnedMesh|SetSkinnedAssetandUpdate _railmount "/Game/AKM/Meshes/Parts/SK_AK_RailAdapter.SK_AK_RailAdapter" true))
    (:1
      (Components|SkinnedMesh|SetSkinnedAssetandUpdate _scope 0 true)
      (Components|SkinnedMesh|SetSkinnedAssetandUpdate _railmount 0 true))))

(fn MagChanged
  (params (Idx :type Integer))
  (bind _magazine (Variables|Default|GetMagazine))
  (switch int Idx
    (:0
      (Components|SkinnedMesh|SetSkinnedAssetandUpdate _magazine "/Game/AKM/Meshes/Parts/SK_AK_Magazine.SK_AK_Magazine" true))
    (:1
      (Components|SkinnedMesh|SetSkinnedAssetandUpdate _magazine "/Game/AKM/Meshes/Parts/SK_AK_DrumMag.SK_AK_DrumMag" true))
    (:2
      (Components|SkinnedMesh|SetSkinnedAssetandUpdate _magazine "/Game/AKM/Meshes/Parts/SK_AK_Magazine_6L.SK_AK_Magazine_6L" true))))

(fn HandguardChanged
  (params (NewIdx :type Integer))
  (bind _handguard (Variables|Default|GetHandguard))
  (switch int NewIdx
    (:0
      (Components|SkinnedMesh|SetSkinnedAssetandUpdate _handguard "/Game/AKM/Meshes/Parts/SK_AK_Handguard_Wood.SK_AK_Handguard_Wood" true))
    (:1
      (Components|SkinnedMesh|SetSkinnedAssetandUpdate _handguard "/Game/AKM/Meshes/Parts/SK_AK_Handguard_B10.SK_AK_Handguard_B10" true))
    (:2
      (Components|SkinnedMesh|SetSkinnedAssetandUpdate _handguard "/Game/AKM/Meshes/Parts/SK_AK_Handguard_Dong.SK_AK_Handguard_Dong" true))
    (:3
      (Components|SkinnedMesh|SetSkinnedAssetandUpdate _handguard "/Game/AKM/Meshes/Parts/SK_AK_Handguard_Shark.SK_AK_Handguard_Shark" true))))

(fn StockChanged
  (params (Idx :type Integer))
  (bind _stock (Variables|Default|GetStock))
  (switch int Idx
    (:0
      (Components|SkinnedMesh|SetSkinnedAssetandUpdate _stock "/Game/AKM/Meshes/Parts/SK_AK_Stock_Wood.SK_AK_Stock_Wood" true))
    (:1
      (Components|SkinnedMesh|SetSkinnedAssetandUpdate _stock 0 true))))