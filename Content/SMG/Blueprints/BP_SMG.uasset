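; BP_SMG is a customizable SMG actor for a weapon configurator viewed through a level CineCamera with mouse input.
; On BeginPlay it creates WBP_MainUI and binds its scope, foregrip and stock change events.
; Scope and stock options set or clear the scope and sling meshes.
; Grip options toggle visibility by swapping an invisible material between two named slots on the base weapon.
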(event EventBeginPlay
  (bind _returnvalue (Game|GetPlayerController 0))
  (CallFunction|UISetup)
  (bind _outactors (Actor|GetAllActorsOfClass "/Script/CinematicCamera.CineCameraActor"))
  (Game|Player|SetViewTargetwithBlend (Game|GetPlayerController 0) (Utilities|Array|Get(acopy) _outactors) 0.0 "VTBlend_Linear" 0.0 false)
  (Variables|/Script/Engine.PlayerController|SetbShowMouseCursor _returnvalue true)
  (Input|SetInputModeGameandUI _returnvalue 0 "DoNotLock" true))

(fn ConstructionScript)

(fn UISetup
  (bind _returnvalue (UserInterface|CreateWidget "/Game/SMG/UI/Widgets/WBP_MainUI.WBP_MainUI_C" (Game|GetPlayerController 0)))
  (UserInterface|Viewport|AddtoViewport _returnvalue 0)
  (EventDispatchers|BindEventtoScopeChanged _returnvalue (EventDispatchers|CreateEvent :!event ScopeChanged))
  (EventDispatchers|BindEventtoForegripChanged _returnvalue (EventDispatchers|CreateEvent :!event GripChanged))
  (EventDispatchers|BindEventtoStockChanged _returnvalue (EventDispatchers|CreateEvent :!event StockChanged)))

(fn ScopeChanged
  (params (Idx :type Integer))
  (bind _sm_scope (Variables|Default|GetSM_Scope))
  (switch int Idx
    (:0
      (Components|StaticMesh|SetStaticMesh _sm_scope "/Game/SMG/Meshes/SM_ACOG.SM_ACOG"))
    (:1
      (Components|StaticMesh|SetStaticMesh _sm_scope 0))))

(fn GripChanged
  (params (NewIdx :type Integer))
  (bind _baseweapon (Variables|Default|GetBaseWeapon))
  (bind _baseweapon_2 (Variables|Default|GetBaseWeapon))
  (switch int NewIdx
    (:0
      (Rendering|Material|SetMaterialbyName _baseweapon_2 "VertGrip" "/Game/SMG/Materials/MI_TacticalGrip.MI_TacticalGrip")
      (Rendering|Material|SetMaterialbyName _baseweapon "Grip" "/Game/SMG/Materials/Master/M_Invis.M_Invis"))
    (:1
      (Rendering|Material|SetMaterialbyName _baseweapon_2 "VertGrip" "/Game/SMG/Materials/Master/M_Invis.M_Invis")
      (Rendering|Material|SetMaterialbyName _baseweapon "Grip" "/Game/SMG/Materials/MI_TacticalGrip.MI_TacticalGrip"))))

(fn StockChanged
  (params (Idx :type Integer))
  (bind _sling (Variables|Default|GetSling))
  (switch int Idx
    (:0
      (Class|SkinnedMeshComponent|SetSkeletalMesh _sling 0 true))
    (:1
      (Class|SkinnedMeshComponent|SetSkeletalMesh _sling "/Game/SMG/Meshes/IndividualParts/SK_SMG_Stock_Sling.SK_SMG_Stock_Sling" true))))