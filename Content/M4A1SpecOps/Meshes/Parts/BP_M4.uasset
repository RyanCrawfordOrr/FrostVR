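; BP_M4 is an M4 rifle Blueprint for an attachment customization display, driven by an on-screen UI.
; On BeginPlay it creates WBP_MainUI, switches the view to the first CineCameraActor found and enables mouse input.
; Widget events drive handlers that show the scope, foregrip, laser or stock when IsA is false and hide it otherwise.
; Showing the laser also plays a 2D sound.
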(event EventBeginPlay
  (bind _returnvalue (Game|GetPlayerController 0))
  (CallFunction|UISetup)
  (bind _outactors (Actor|GetAllActorsOfClass "/Script/CinematicCamera.CineCameraActor"))
  (Game|Player|SetViewTargetwithBlend (Game|GetPlayerController 0) (Utilities|Array|Get(acopy) _outactors) 0.0 "VTBlend_Linear" 0.0 false)
  (Variables|/Script/Engine.PlayerController|SetbShowMouseCursor _returnvalue true)
  (Input|SetInputModeGameandUI _returnvalue 0 "DoNotLock" true false))

(fn ConstructionScript)

(fn UISetup
  (bind _returnvalue (UserInterface|CreateWidget "/Game/M4A1SpecOps/UI/Widgets/WBP_MainUI.WBP_MainUI_C" (Game|GetPlayerController 0)))
  (UserInterface|Viewport|AddtoViewport _returnvalue 0)
  (EventDispatchers|BindEventtoScopeChanged _returnvalue (EventDispatchers|CreateEvent :!event ScopeChanged))
  (EventDispatchers|BindEventtoForegripChanged _returnvalue (EventDispatchers|CreateEvent :!event GripChanged))
  (EventDispatchers|BindEventtoLaserChanged _returnvalue (EventDispatchers|CreateEvent :!event LaserChanged))
  (EventDispatchers|BindEventtoStockChanged _returnvalue (EventDispatchers|CreateEvent :!event StockChanged)))

(fn ScopeChanged
  (params (IsA :type Boolean))
  (Rendering|SetVisibility (Variables|Default|GetScope) (not IsA) false))

(fn StockChanged
  (params (IsA :type Boolean))
  (Rendering|SetVisibility (Variables|Default|GetStock) (not IsA) false))

(fn LaserChanged
  (params (IsA :type Boolean))
  (Rendering|SetVisibility (Variables|Default|GetLaser) (not IsA) false)
  (if (not IsA)
    (Audio|PlaySound2D "/Game/M4A1SpecOps/Sounds/SC_Laser.SC_Laser" 1.0 1.0 0.0 0 0)))

(fn GripChanged
  (params (IsA :type Boolean))
  (Rendering|SetVisibility (Variables|Default|GetForegrip) (not IsA) false))